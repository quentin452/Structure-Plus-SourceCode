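; Tek sloped gate wedge piece for tree platforms, a structure that can be made immune to damage by server config.
; On construction outside dedicated servers, it creates a dynamic material instance and zeroes the world position offset limits.
; At begin play, non-preview structures on the authority cache the platform immunity setting from the game mode.
; BPAdjustDamage returns zero damage when immune, otherwise the incoming damage.
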(fn `BPAdjustDamage`
  (params (IncomingDamage :type "Float (double-precision)") (TheDamageEvent :type "EngineTypes.DamageEvent Structure") (EventInstigator :type "Controller Object Reference") (DamageCauser :type "Actor Object Reference") (bIsPointDamage :type Boolean) (PointHitInfo :type "EngineTypes.HitResult Structure"))
  (returns (ReturnValue :type "Float (double-precision)"))
  (return (`KismetMathLibrary.SelectFloat` 0.0 IncomingDamage (`self.IsImmune`))))

(fn `ReceiveBeginPlay`
  (`parent.ReceiveBeginPlay`)
  (if (not (`self.bIsPreviewStructure`))
    (`/Engine/EditorBlueprintResources/ActorMacros.Switch Has Authority`
      (:`Authority`
        (bind _value (`/Game/Mods/StructuresPlusMod/_Scripts/ConfigFunctions.SP_GetConfig_-_Bool` (`GameplayStatics.GetGameMode`) "ArePlatformsImmuneToDamage"))
        (set `self.IsImmune` _value)))))

(fn `UserConstructionScript`
  (bind _mystaticmesh (`self.MyStaticMesh`))
  (`parent.UserConstructionScript`)
  (if (not (`KismetSystemLibrary.IsDedicatedServer`))
    (bind _returnvalue (`PrimitiveComponent.CreateDynamicMaterialInstance` _mystaticmesh 0 (`PrimitiveComponent.GetMaterial` _mystaticmesh 0)))
    (`MaterialInstanceDynamic.SetScalarParameterValue` _returnvalue "WPO offset max" 0.0)
    (`MaterialInstanceDynamic.SetScalarParameterValue` _returnvalue "WPO offset min" 0.0)))