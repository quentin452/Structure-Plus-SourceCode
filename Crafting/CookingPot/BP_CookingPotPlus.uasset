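; Structures Plus style cooking pot for ARK that reads its inventory slot count and crafting speed from game mode config on the server.
; A tertiary inventory button cycles autocrafting between everything, all except dyes, and disabled.
; OnRep_AutoCraftMode applies the mode through the inventory's autocraft check and per-item flags on built-in dye blueprints.
; It also overrides one placement rejection code and limits activation to the owning team while locked.
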(fn `BPCanBeActivatedByPlayer`
  (params (PC :type "ShooterPlayerController Object Reference"))
  (returns (ReturnValue :type Boolean))
  (return (or (== (`Actor.TargetingTeam` PC) (`self.TargetingTeam`)) (not (`self.bIsLocked`)))))

(fn `BPGetMultiUseEntries`
  (params (ForPC :type "PlayerController Object Reference") (MultiUseEntries :type "Array of Actor.MultiUseEntry Structure (by ref)"))
  (returns (ReturnValue :type "Array of Actor.MultiUseEntry Structure"))
  (bind _entriesout (`/Game/Mods/StructuresPlusMod/_Scripts/MultiUseMenuFunctions.SP_Update_Multi_Use_Menu` ForPC MultiUseEntries self))
  (`|ExecutionSequence`
    (:`then_0`
      (bind _returnvalue (`self.AllowStructureAccess` ForPC))
      (if _returnvalue
        (`KismetArrayLibrary.Array_Add` _entriesout (make `Actor.MultiUseEntry` :`UseString` (select `int` (`self.AutoCraftMode`) :`0` "Autocrafting Everything" :`1` "Autocrafting All Except Dyes" :`2` "Autocrafting Disabled") :`UseIndex` 9001 :`Priority` -1020 :`bHideFromUI` true :`bDisplayOnInventoryUITertiary` true))))
    (:`then_1`
      (return _entriesout))))

(fn `BPIsAllowedToBuild`
  (params (OutPlacementData :type "PrimalStructure.PlacementData Structure (by ref)") (CurrentAllowedReason :type Integer))
  (returns (ReturnValue :type Integer))
  (return (`KismetMathLibrary.SelectInt` 1 CurrentAllowedReason (== CurrentAllowedReason -9))))

(fn `BPTryMultiUse`
  (params (ForPC :type "PlayerController Object Reference") (UseIndex :type Integer))
  (returns (ReturnValue :type Boolean))
  (bind _returnvalue (+ (`self.AutoCraftMode`) 1))
  (`|ExecutionSequence`
    (:`then_0`
      (if (== UseIndex 601)
        (set `self.IsUnlocked` (not (`self.bIsLocked`)))
        (elif (== UseIndex 9001)
          (set `self.AutoCraftMode` (`KismetMathLibrary.SelectInt` 0 _returnvalue (> _returnvalue 2)) true))))
    (:`then_1`
      (return true))))

(fn `OnRep_AutoCraftMode`
  (bind _myinventorycomponent (`self.MyInventoryComponent`))
  (switch `int` (`self.AutoCraftMode`)
    (:`0`
      (set `PrimalInventoryComponent.bCheckForAutoCraftBlueprints` true _myinventorycomponent)
      (`self.ToggleDyeAutoCrafting` true))
    (:`1`
      (`self.ToggleDyeAutoCrafting` false))
    (:`2`
      (set `PrimalInventoryComponent.bCheckForAutoCraftBlueprints` false _myinventorycomponent))))

(fn `OnRep_InventorySlots`
  (set `PrimalInventoryComponent.MaxInventoryItems` (`self.InventorySlots`) (`self.MyInventoryComponent`)))

(fn `ReceiveBeginPlay`
  (bind _returnvalue (`GameplayStatics.GetGameMode`))
  (`parent.ReceiveBeginPlay`)
  (if (not (`self.bIsPreviewStructure`))
    (`/Engine/EditorBlueprintResources/ActorMacros.Switch Has Authority`
      (:`Authority`
        (`|ExecutionSequence`
          (:`then_0`
            (bind _value (`/Game/Mods/StructuresPlusMod/_Scripts/ConfigFunctions.SP_GetConfigSetting_-_InventorySize` _returnvalue "CookingPotSlotCount" 25))
            (set `self.InventorySlots` _value true))
          (:`then_1`
            (bind _value_2 (`/Game/Mods/StructuresPlusMod/_Scripts/ConfigFunctions.SP_GetConfigSetting_-_CraftingSpeed` _returnvalue "CookingPotCraftingSpeed"))
            (set `PrimalInventoryComponent.CraftingItemSpeed` _value_2 (`self.MyInventoryComponent`)))
          (:`then_2`
            (set `self.bIsLocked` (not (`self.IsUnlocked`)) true))
          (:`then_3`
            (`/Engine/EditorBlueprintResources/ActorMacros.SwitchNetAuthority`
              (:`PlayerServer`
                (`self.OnRep_AutoCraftMode`)))))))))

(fn `ToggleDyeAutoCrafting`
  (params (Enable :type Boolean))
  (for _array_element (`PrimalInventoryComponent.InventoryItems` (`self.MyInventoryComponent`))
    (bind _asprimalitemdyegeneric_c (cast `/Game/PrimalEarth/CoreBlueprints/Items/PrimalItemDyeGeneric` _array_element))
    (if (and (`PrimalItem.bIsBlueprint` _array_element) (not (`PrimalItem.bAllowRemovalFromInventory` _array_element)))
      (set `PrimalItem.bAutoCraftBlueprint` Enable _asprimalitemdyegeneric_c))))

(fn `UserConstructionScript`
  (`parent.UserConstructionScript`))