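; S+ Tek crop plot structure that keeps itself watered and grows faster or slower depending on whether it is powered.
; Water refills to maximum whenever it drops below half, checked at begin play and on growth-multiplier queries.
; Inventory changes or item use in early phases check for fertilized "MeatSeed" crops, fast-forwarding them by shrinking the refresh interval to one frame.
; A timer derived from summed phase thresholds then restores a random interval.
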(fn ConstructionScript
  (|CallParentFunction))

(fn BPGetAdditionalGrowthMultiplier
  (CallFunction|UpdateWaterAmt)
  (return (Math|Float|SelectFloat (Variables|Default|GetPoweredGrowthModifier) (Variables|Default|GetUnpoweredGrowthModifier) (Variables|Default|GetbIsPowered))))

(fn BPNotifyInventoryItemChange
  (params (bIsItemAdd :type Boolean) (theItem :type Primal%20Item%20Object%20Reference) (bEquipItem :type Boolean))
  (Class|KismetSystemLibrary|IsRunningonServer
    (:Yes
      (if (< (Variables|Default|GetCurrentCropPhase) (Math|Byte|MakeLiteralByte 3))
        (Class|KismetSystemLibrary|SetTimerforNextTick 0 "CheckInstantGrow" false)))))

(fn CheckInstantGrow
  (bind _myinventorycomponent (Variables|Default|GetMyInventoryComponent))
  (if (Math|Boolean|ANDBoolean (Variables|Default|GetbIsSeeded) (> (Variables|Default|GetWaterAmount) 0.0) (> (Variables|Default|GetFertilizerAmount) 0))
    (Utilities|IsValid _myinventorycomponent
      (:Is%20Valid
        (bind _returnvalue (Class|PrimalInventoryComponent|FindAllItemsOfType _myinventorycomponent (Variables|Default|GetSeedBaseItemTemplate) false true false false false false false))
        (if (Utilities|Array|IsValidIndex _returnvalue)
          (if (Utilities|Name|Equal(Name) (Variables|/Script/ShooterGame.PrimalItem|GetCustomTag (Utilities|Array|Get(acopy) _returnvalue)) "MeatSeed")
            (for _array_element (Variables|/Script/ShooterGame.PrimalItem|GetCropPhasesData (Utilities|Array|Get(acopy) _returnvalue))
              (LocalVariables|SetLocalTimer (+ (LocalVariables|GetLocalTimer) (.NextStageFertilizerCacheThreshold (Utilities|Struct|BreakCropItemPhaseData _array_element)))))
            (Variables|Default|SetLastCropRefreshTime (Class|VictoryCore|GetNetworkTimeinSeconds))
            (Variables|Default|SetCropRefreshInterval (Utilities|Time|GetWorldDeltaSeconds))
            (Utilities|Time|SetTimerbyFunctionName 0 "ResetRefreshInterval" (+ (LocalVariables|GetLocalTimer) 1.0))))))))

(fn BPInventoryItemUsed
  (params (InventoryItemObject :type Object%20Object%20Reference))
  (if (< (Variables|Default|GetCurrentCropPhase) (Math|Byte|MakeLiteralByte 3))
    (Class|KismetSystemLibrary|SetTimerforNextTick 0 "CheckInstantGrow" false)))

(fn ResetRefreshInterval
  (Variables|Default|SetCropRefreshInterval (Math|Random|RandomFloatinRange (Variables|Default|GetCropRefreshIntervalMin) (Variables|Default|GetCropRefreshIntervalMax))))

(fn ReceiveBeginPlay
  (|CallParentFunction)
  (if (not (Variables|Default|GetbIsPreviewStructure))
    (Networking|SwitchHasAuthority
      (:Authority
        (CallFunction|UpdateWaterAmt)))))

(fn UpdateWaterAmt
  (bind _maxwateramount (Variables|Default|GetMaxWaterAmount))
  (bind _wateramount (Variables|Default|GetWaterAmount))
  (if (< _wateramount (/ _maxwateramount 2.0))
    (Class|PrimalStructureItemContainerCropPlot|AddWater (- _maxwateramount _wateramount) true)))