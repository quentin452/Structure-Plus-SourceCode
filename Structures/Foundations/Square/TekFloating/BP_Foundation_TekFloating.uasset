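; Floating Tek square foundation structure that can only be placed on the surface of water.
; When the current build reason is positive, it samples just above and below the placement location, requiring dry above and underwater below, else returning a custom failure code with its own message.
; A snap-point filter blocks certain indices for any child structure and others only for another floating Tek foundation of the same class.
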(fn ConstructionScript
  (|CallParentFunction))

(fn ReceiveBeginPlay)

(fn IsValidSnapPointto
  (params (ChildStructure :type Primal%20Structure%20Object%20Reference) (MySnapPointToIndex :type Integer))
  (LocalVariables|SetAllowSnapTo true)
  (Utilities|FlowControl|Sequence
    (:then_0
      (if (Math|Boolean|ORBoolean (== MySnapPointToIndex 76) (== MySnapPointToIndex 78) (== MySnapPointToIndex 80) (== MySnapPointToIndex 82))
        (LocalVariables|SetAllowSnapTo false)
        (elif (and (or (== MySnapPointToIndex 73) (== MySnapPointToIndex 74)) (== (Utilities|GetClass ChildStructure) "BP_Foundation_TekFloating_C"))
          (LocalVariables|SetAllowSnapTo false))))
    (:then_1
      (return (LocalVariables|GetAllowSnapTo)))))

(fn BPIsAllowedtoBuild
  (params (OutPlacementData :type Placement%20Data%20Structure%20%28by%20ref%29) (CurrentAllowedReason :type Integer))
  (bind _adjustedlocation (Utilities|Struct|BreakPlacementData OutPlacementData))
  (bind _returnvalue (Class|Actor|GetWorld))
  (LocalVariables|SetAllowReason CurrentAllowedReason)
  (Utilities|FlowControl|Sequence
    (:then_0
      (if (> (LocalVariables|GetAllowReason) 0)
        (bind _returnvalue_2 (Class|BiomeZoneVolume|IsPointUnderwater _returnvalue (+ _adjustedlocation "0, 0,50.000000") true 0.0 false true))
        (bind _returnvalue_3 (Class|BiomeZoneVolume|IsPointUnderwater _returnvalue (- _adjustedlocation "0, 0,50.000000") true 0.0 false true))
        (if (not (and (not _returnvalue_2) _returnvalue_3))
          (LocalVariables|SetAllowReason -876))))
    (:then_1
      (return (LocalVariables|GetAllowReason)))))

(fn BPOverrideCantBuildReasonString
  (params (CantBuildReason :type Integer))
  (return (Utilities|String|SelectString "Can only be placed on the surface of water." "" (== CantBuildReason -876))))