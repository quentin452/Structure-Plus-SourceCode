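; Triangle glass foundation structure whose transparency and edge model can be changed through a glass interface.
; Construction gives the inside and outside faces their own dynamic glass materials, skipped for previews and dedicated servers.
; Replicated settings and model index apply visuals through RepNotify helpers, skipped on dedicated servers and called directly on player-hosted servers at BeginPlay.
; The authority reads minimum opacity from game-mode config and raises lower values to it.
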(event `self.IGlassSetModel`
  (params (ModelIndex :type Integer))
  (set `self.ModelIndex` ModelIndex true))

(event `self.IGlassSetTransparency`
  (params (GlassSetting :type "/Game/Mods/StructuresPlusMod/_Structs/SPGlassSettings Structure"))
  (set `self.GlassSettings` GlassSetting true))

(fn `IGlassGetModel`
  (returns (ModelIndex :type Integer) (IsTriangle :type Boolean))
  (return (`self.ModelIndex`) true))

(fn `IGlassGetPreventReason`
  (returns (PreventReason :type String))
  (return ""))

(fn `IGlassGetTransparency`
  (returns (GlassSettings :type "/Game/Mods/StructuresPlusMod/_Structs/SPGlassSettings Structure") (MinOpacity :type "Float (double-precision)"))
  (return (`self.GlassSettings`) (`self.MinOpacity`)))

(fn `OnRep_GlassSettings`
  (if (not (`KismetSystemLibrary.IsDedicatedServer`))
    (`/Game/Mods/StructuresPlusMod/_Scripts/GlassFunctions.SP_Glass_-_SetTransparency` (`self.GlassSettings`) (`self.InsideMIC`) (`self.OutsideMIC`))))

(fn `OnRep_MinOpacity`
  (bind _minopacity (`self.MinOpacity`))
  (bind (_glasssettings_transparencytype _glasssettings_opacity) (break `/Game/Mods/StructuresPlusMod/_Structs/SPGlassSettings` (`self.GlassSettings`)))
  (`/Engine/EditorBlueprintResources/ActorMacros.Switch Has Authority`
    (:`Authority`
      (if (< _glasssettings_opacity _minopacity)
        (set `self.GlassSettings` (make `/Game/Mods/StructuresPlusMod/_Structs/SPGlassSettings` _glasssettings_transparencytype _minopacity) true)))))

(fn `OnRep_ModelIndex`
  (if (not (`KismetSystemLibrary.IsDedicatedServer`))
    (`/Game/Mods/StructuresPlusMod/_Scripts/GlassFunctions.SP_Glass_-_SetModel` (`self.ModelIndex`) null (`self.GlassBackMesh`) (`self.GlassLeftMesh`) (`self.GlassRightMesh`) true)))

(fn `ReceiveBeginPlay`
  (`parent.ReceiveBeginPlay`)
  (if (not (`self.bIsPreviewStructure`))
    (`/Engine/EditorBlueprintResources/ActorMacros.Switch Has Authority`
      (:`Authority`
        (bind _value (`/Game/Mods/StructuresPlusMod/_Scripts/ConfigFunctions.SP_GetConfig_-_Float` (`GameplayStatics.GetGameMode`) "MinimumGlassTransparency" 0.0 0.0 1.0))
        (set `self.MinOpacity` _value true)
        (`/Engine/EditorBlueprintResources/ActorMacros.SwitchNetAuthority`
          (:`PlayerServer`
            (`self.OnRep_GlassSettings`)
            (`self.OnRep_ModelIndex`)))))))

(fn `UserConstructionScript`
  (bind _mystaticmesh (`self.MyStaticMesh`))
  (`parent.UserConstructionScript`)
  (if (not (or (`self.bIsPreviewStructure`) (`KismetSystemLibrary.IsDedicatedServer`)))
    (bind _returnvalue (`KismetMaterialLibrary.CreateDynamicMaterialInstance` "/Game/PrimalEarth/StructuresPlus/_Materials/GlassMIC.GlassMIC"))
    (set `self.InsideMIC` _returnvalue)
    (bind _returnvalue_2 (`KismetMaterialLibrary.CreateDynamicMaterialInstance` "/Game/PrimalEarth/StructuresPlus/_Materials/GlassMIC.GlassMIC"))
    (set `self.OutsideMIC` _returnvalue_2)
    (`PrimitiveComponent.SetMaterial` _mystaticmesh 0 (`self.InsideMIC`))
    (`PrimitiveComponent.SetMaterial` _mystaticmesh 1 (`self.OutsideMIC`))))