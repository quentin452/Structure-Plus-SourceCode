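; Sloped underwater cube compartment for Structures Plus, a vacuum structure that gives characters entering its protection box radiation and liquid protection buffs.
; Multi-use menus, gated by access level, toggle side locking and flooding, drain or flood compartments, and spawn emitters on flood changes.
; Placement overrides govern snapping and what attaches, marking snapped or linked structures as foundations.
; Global and INI settings can restrict placement to water, destroying above-water compartments on begin play.
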(event OnComponentBeginOverlap(RadiationProtectionBox)
  (params (OtherActor :type Actor%20Object%20Reference) (OtherComp :type Primitive%20Component%20Object%20Reference) (OtherBodyIndex :type Integer) (bFromSweep :type Boolean) (SweepResult :type Hit%20Result%20Structure%20%28by%20ref%29))
  (Networking|SwitchHasAuthority
    (:Authority
      (bind _asprimalcharacter (Utilities|Casting|CastToPrimalCharacter OtherActor))
      (Utilities|FlowControl|Sequence
        (:then_0
          (bind _returnvalue (Class|PrimalCharacter|HasBuff _asprimalcharacter "/Game/Mods/StructuresPlusMod/_Buffs/Buff_StructuresPlus_RadiationProtection.Buff_StructuresPlus_RadiationProtection_C" true))
          (if (not _returnvalue)
            (Class|PrimalBuff|StaticAddBuff "/Game/Mods/StructuresPlusMod/_Buffs/Buff_StructuresPlus_RadiationProtection.Buff_StructuresPlus_RadiationProtection_C" _asprimalcharacter 0 0 false)))
        (:then_1
          (bind _returnvalue_2 (Class|PrimalCharacter|HasBuff _asprimalcharacter "/Game/Mods/StructuresPlusMod/_Buffs/Buff_StructuresPlus_LiquidProtection.Buff_StructuresPlus_LiquidProtection_C" true))
          (if (not _returnvalue_2)
            (Class|PrimalBuff|StaticAddBuff "/Game/Mods/StructuresPlusMod/_Buffs/Buff_StructuresPlus_LiquidProtection.Buff_StructuresPlus_LiquidProtection_C" _asprimalcharacter 0 0 false)))))))

(fn ConstructionScript
  (|CallParentFunction)
  (if (Variables|Default|GetbIsPreviewStructure)
    (bind _assplusglobalactor_c (Utilities|Casting|CastToSPlusGlobalActor (CallFunction|SPGetGlobalActor self)))
    (Variables|Default|SetbOnlyAllowPlacementInWater (Variables|/Game/Mods/StructuresPlusMod/SPlusGlobalActor.SPlusGlobalActor_C|GetDisableUnderwaterAboveWater _assplusglobalactor_c))))

(fn ChangedCompartmentFloodState
  (if (Variables|Default|GetAllowFlooding)
    (if (not (Networking|IsDedicatedServer))
      (if (> (Class|VictoryCore|TimeSince (Class|Actor|GetWorld) (Variables|Default|GetCreationTime)) 0.33)
        (Game|SpawnActorfromClass (select (Variables|Default|GetbIsFlooded) "/Game/PrimalEarth/General/UnderwaterBaseFloodedEmitter.UnderwaterBaseFloodedEmitter_C" "/Game/PrimalEarth/General/UnderwaterBaseUnfloodedEmitter.UnderwaterBaseUnfloodedEmitter_C") (Transformation|GetActorTransform) true)))
    (else
      (Class|KismetSystemLibrary|IsRunningonServer
        (:Yes
          (if (Variables|Default|GetbIsFlooded)
            (Variables|Default|SetbIsFlooded false true)))))))

(fn BPForceConsideredEnemyFoundation
  (params (PC :type Player%20Controller%20Object%20Reference) (ForNewStructure :type Primal%20Structure%20Object%20Reference) (TestAtLocation :type Vector%20%28by%20ref%29 :default "0, 0, 0"))
  (return true))

(fn BPPreventPlacingStructureOntoMe
  (params (PC :type Player%20Controller%20Object%20Reference) (ForNewStructure :type Primal%20Structure%20Object%20Reference) (ForHitResult :type Hit%20Result%20Structure%20%28by%20ref%29))
  (bind (_location _normal _impactpoint _impactnormal _physmat _hitactor _hitcomponent) (Collision|BreakHitResult ForHitResult))
  (bind _requireswall (CallFunction|SPRequiresWallAttachforUnderwater self _location))
  (return (and (not _requireswall) (Math|Boolean|ORBoolean (== _hitcomponent 0) (== _hitcomponent (Variables|Default|GetCollision_Front)) (== _hitcomponent (Variables|Default|GetCollision_Left)) (== _hitcomponent (Variables|Default|GetCollision_Right)) (== _hitcomponent (Variables|Default|GetCollision_Back))))))

(fn BPGetMultiUseEntries
  (params (ForPC :type Player%20Controller%20Object%20Reference) (MultiUseEntries :type Array%20of%20Multi%20Use%20Entry%20Structures))
  (bind _self self)
  (bind _entriesout (CallFunction|SPUpdateMultiUseMenu ForPC MultiUseEntries _self false false false false))
  (Utilities|FlowControl|Sequence
    (:then_0
      (bind _accesslevel (CallFunction|SPGetAccessLevel ForPC _self))
      (CallFunction|SPCleanUpVacuumCompartmentMenu _entriesout _self (and (>= _accesslevel 2) (not (Variables|Default|GetLockSides))))
      (if (>= _accesslevel 2)
        (Utilities|Array|Add _entriesout (Utilities|Struct|MakeMultiUseEntry (Utilities|String|SelectString "Allow Side Change" "Prevent Side Change" (Variables|Default|GetLockSides)) 9001 -1002))
        (Utilities|Array|Add _entriesout (Utilities|Struct|MakeMultiUseEntry "[Water Management]" 9100 -1000 true true true (Math|Conversions|ToColor(LinearColor) (CallFunction|SPGetMultiUseSpecialColor))))
        (Utilities|Array|Add _entriesout (Utilities|Struct|MakeMultiUseEntry (Utilities|String|SelectString "Prevent Flooding" "Allow Flooding" (Variables|Default|GetAllowFlooding)) 9002 1000 9100))
        (Utilities|Array|Add _entriesout (Utilities|Struct|MakeMultiUseEntry -1 500 true true 9100))
        (Utilities|Array|Add _entriesout (Utilities|Struct|MakeMultiUseEntry "Drain All Connected" 9003 0 9100))
        (if (Variables|Default|GetbIsFlooded)
          (Utilities|Array|Add _entriesout (Utilities|Struct|MakeMultiUseEntry "Drain Water" 9004 -500 9100))
          (elif (Variables|Default|GetAllowFlooding)
            (Utilities|Array|Add _entriesout (Utilities|Struct|MakeMultiUseEntry "Flood Compartment" 9005 -500 9100))
            (else
              (Utilities|Array|Add _entriesout (Utilities|Struct|MakeMultiUseEntry -1 -500 true true 9100)))))))
    (:then_1
      (return _entriesout))))

(fn BPTryMultiUse
  (params (ForPC :type Player%20Controller%20Object%20Reference) (UseIndex :type Integer))
  (Utilities|FlowControl|Sequence
    (:then_0
      (switch int UseIndex
        (:Default
          (if (or (and (>= UseIndex 42) (<= UseIndex 47)) (and (>= UseIndex 72) (<= UseIndex 77)))
            (CallFunction|SPNormalizeConnectedPorthole ForPC self UseIndex)))
        (:9001
          (Variables|Default|SetLockSides (not (Variables|Default|GetLockSides)) true))
        (:9002
          (Variables|Default|SetAllowFlooding (not (Variables|Default|GetAllowFlooding)) true))
        (:9003
          (CallFunction|SPDrainAllConnectedCompartments self))
        (:9004
          (Variables|Default|SetbIsFlooded false true))
        (:9005
          (Variables|Default|SetbIsFlooded true true))))
    (:then_1
      (return true))))

(fn IsValidSnapPointto
  (params (ChildStructure :type Primal%20Structure%20Object%20Reference) (MySnapPointToIndex :type Integer))
  (Variables|/Script/ShooterGame.PrimalStructure|SetbIsFoundation ChildStructure true false)
  (return true))

(fn BPIsAllowedtoBuild
  (params (OutPlacementData :type Placement%20Data%20Structure%20%28by%20ref%29) (CurrentAllowedReason :type Integer))
  (return (Math|Integer|SelectInt 1 CurrentAllowedReason (== CurrentAllowedReason -9))))

(fn BPOverrideSnappedtoTransform
  (params (childStructure :type Primal%20Structure%20Object%20Reference) (ChildSnapFromIndex :type Integer) (ChildSnapFromName :type Name :default "None") (UnsnappedPlacementPos :type Vector :default "0, 0, 0") (UnsnappedPlacementRot :type Rotator :default "0, 0, 0") (SnappedPlacementPos :type Vector :default "0, 0, 0") (SnappedPlacementRot :type Rotator :default "0, 0, 0") (SnapToIndex :type Integer) (SnapToName :type Name :default "None"))
  (return (- SnappedPlacementPos (Math|Vector|SelectVector "0, 0,-60.000000" "0, 0,60.000000" (Math|Float|InRange(Float) (.roll (Transformation|GetActorRotation)) -1.0 1.0))) SnappedPlacementRot 0 (or (== SnapToIndex 43) (== SnapToIndex 44))))

(fn ReceiveBeginPlay
  (|CallParentFunction)
  (Utilities|FlowControl|Sequence
    (:then_0
      (bind _assplusglobalactor_c (Utilities|Casting|CastToSPlusGlobalActor (CallFunction|SPGetGlobalActor self)))
      (if (Variables|/Game/Mods/StructuresPlusMod/SPlusGlobalActor.SPlusGlobalActor_C|GetNoFoundationsRequired _assplusglobalactor_c)
        (Variables|Default|SetbForcePlacingOnGround false)
        (Variables|Default|SetbSnapRequiresPlacementOnGround false)))
    (:then_1
      (if (not (Variables|Default|GetbIsPreviewStructure))
        (Networking|SwitchHasAuthority
          (:Authority
            (Utilities|FlowControl|Sequence
              (:then_0
                (bind _asshootergamemode (Utilities|Casting|CastToShooterGameMode (Game|GetGameMode)))
                (bind _returnvalue (Class|ShooterGameMode|GetBoolOptionIni _asshootergamemode "StructuresPlus" "DisableAbilityToPlaceVacuumCompartmentsAboveWater" false))
                (if _returnvalue
                  (bind _returnvalue_2 (Class|BiomeZoneVolume|IsPointUnderwater (Class|Actor|GetWorld) (Transformation|GetActorLocation) true 0.0 true false))
                  (if (not _returnvalue_2)
                    (Actor|DestroyActor))))
              (:then_1
                (for _array_element (Variables|Default|GetLinkedStructures)
                  (Variables|/Script/ShooterGame.PrimalStructure|SetbIsFoundation _array_element true false))))))))))

(fn BPServerHandleNetExecCommand
  (params (FromPC :type Player%20Controller%20Object%20Reference) (CommandName :type Name :default "None") (ExecParams :type BP%20Net%20Exec%20Params%20Structure%20%28by%20ref%29))
  (Utilities|FlowControl|Sequence
    (:then_0
      (switch name CommandName
        (:ToggleSideLock
          (Variables|Default|SetLockSides (not (Variables|Default|GetLockSides)) true)
          (Class|StructuresPlus|SPMessageClient FromPC (Utilities|String|SelectString "Compartment configuration locked." "Compartment configuration unlocked." (Variables|Default|GetLockSides)) "Default"))))
    (:then_1
      (return true))))

(fn BPClientDoMultiUse
  (params (ForPC :type Player%20Controller%20Object%20Reference) (ClientUseIndex :type Integer))
  (bind _asshooterplayercontroller (Utilities|Casting|CastToShooterPlayerController ForPC))
  (switch int ClientUseIndex
    (:9100
      (Class|ShooterPlayerController|SetMultiUseWheelCategory _asshooterplayercontroller ClientUseIndex))))