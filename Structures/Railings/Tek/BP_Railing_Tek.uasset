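; Tek-tier railing structure that changes its visible mesh depending on whether it is placed on a ramp or is a half wall.
; Two RepNotify flags each toggle visibility between the default mesh and a slanted or half-wall variant, then force a net update.
; Each handler sets the default mesh's visibility from its own flag alone, and construction defers to the parent class.
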(fn `OnRep_IsHalfWall`
  (bind _halfwallmesh (`self.HalfWallMesh`))
  (bind _mesh (`self.Mesh`))
  (if (`self.IsHalfWall`)
    (`SceneComponent.SetVisibility` _halfwallmesh true false)
    (`SceneComponent.SetVisibility` _mesh false false)
    (else
      (`SceneComponent.SetVisibility` _halfwallmesh false false)
      (`SceneComponent.SetVisibility` _mesh true false)))
  (`self.ForceNetUpdate` false))

(fn `OnRep_IsPlacedOnRamp`
  (bind _slantedmesh (`self.SlantedMesh`))
  (bind _mesh (`self.Mesh`))
  (if (`self.IsPlacedOnRamp`)
    (`SceneComponent.SetVisibility` _slantedmesh true false)
    (`SceneComponent.SetVisibility` _mesh false false)
    (else
      (`SceneComponent.SetVisibility` _slantedmesh false false)
      (`SceneComponent.SetVisibility` _mesh true false)))
  (`self.ForceNetUpdate` false))

(fn `UserConstructionScript`
  (`parent.UserConstructionScript`))