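; Forcefield wall structure that opens for characters permitted by its access setting, which the use menu cycles between tribe only, allies and none.
; A detector overlap tracks permitted actors, opening the wall for the first and closing it after the last leaves.
; An authority-side next-tick timer interpolates the door cycle value, feeding a dynamic material parameter on player servers and clients.
; The same material takes the structure's paint color.
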(event `self.PawnDetector.OnComponentBeginOverlap`
  (params (OtherActor :type "Actor Object Reference") (OtherComp :type "PrimitiveComponent Object Reference") (OtherBodyIndex :type Integer) (bFromSweep :type Boolean) (SweepResult :type "EngineTypes.HitResult Structure (by ref)"))
  (bind _actorsinforcefield (`self.ActorsInForcefield`))
  (bind _allowaccess (`/Game/Mods/StructuresPlusMod/_Scripts/ForcefieldFunctions.SP_AllowAccessThroughForcefieldWall` OtherActor self (`self.ForcefieldSetting`)))
  (if _allowaccess
    (`|ExecutionSequence`
      (:`then_0`
        (if (== (`KismetArrayLibrary.Array_Length` _actorsinforcefield) 0)
          (`/Game/Mods/StructuresPlusMod/_Scripts/ForcefieldFunctions.SP_HandleForcefieldWallOpenClose` self true)))
      (:`then_1`
        (`/Game/Mods/StructuresPlusMod/_Macros/UtilityMacros.SP_AddIfUnique` _actorsinforcefield OtherActor
          (:`Done`
            (if (== (`self.DoorCycleCurrent`) 1.0)
              (set `self.DoorCycleTarget` 0.0)
              (`/Engine/EditorBlueprintResources/ActorMacros.Switch Has Authority`
                (:`Authority`
                  (`KismetSystemLibrary.K2_SetTimerForNextTick` null "MaterialCycleEvent" true))))))))))

(event `self.PawnDetector.OnComponentEndOverlap`
  (params (OtherActor :type "Actor Object Reference") (OtherComp :type "PrimitiveComponent Object Reference") (OtherBodyIndex :type Integer))
  (bind _actorsinforcefield (`self.ActorsInForcefield`))
  (`KismetArrayLibrary.Array_RemoveItem` _actorsinforcefield OtherActor)
  (if (== (`KismetArrayLibrary.Array_Length` _actorsinforcefield) 0)
    (`/Game/Mods/StructuresPlusMod/_Scripts/ForcefieldFunctions.SP_HandleForcefieldWallOpenClose` self)
    (`/Engine/EditorBlueprintResources/ActorMacros.Switch Has Authority`
      (:`Authority`
        (if (== (`self.DoorCycleCurrent`) 0.0)
          (set `self.DoorCycleTarget` 1.0)
          (`KismetSystemLibrary.K2_SetTimerForNextTick` null "MaterialCycleEvent" true))))))

(event `MaterialCycleEvent`
  (bind _doorcyclecurrent (`self.DoorCycleCurrent`))
  (set `self.DoorCycleCurrent` (`KismetMathLibrary.FInterpTo_Constant` (`self.DoorCycleCurrent`) (`self.DoorCycleTarget`) (`GameplayStatics.GetWorldDeltaSeconds`) 1.75))
  (`|ExecutionSequence`
    (:`then_0`
      (if (== _doorcyclecurrent (`self.DoorCycleTarget`))
        (if (and (== _doorcyclecurrent 0.0) (== (`KismetArrayLibrary.Array_Length` (`self.ActorsInForcefield`)) 0))
          (set `self.DoorCycleTarget` 1.0)
          (else
            (`KismetSystemLibrary.K2_ClearTimer` null "MaterialCycleEvent")))))
    (:`then_1`
      (`self.HandleMaterialCycleEvent` (`self.DoorCycleCurrent`)))))

(event `HandleMaterialCycleEvent`
  (params (DoorValue :type "Float (double-precision)"))
  (`/Engine/EditorBlueprintResources/ActorMacros.SwitchNetAuthority`
    (:`PlayerServer`
      _)
    (:`Client`
      _))
  (`MaterialInstanceDynamic.SetScalarParameterValue` (`self.ForcefieldMat`) "CycleDoor" DoorValue))

(fn `BPGetMultiUseEntries`
  (params (ForPC :type "PlayerController Object Reference") (MultiUseEntries :type "Array of Actor.MultiUseEntry Structure (by ref)"))
  (returns (ReturnValue :type "Array of Actor.MultiUseEntry Structure"))
  (bind _entriesout (`/Game/Mods/StructuresPlusMod/_Scripts/MultiUseMenuFunctions.SP_Update_Multi_Use_Menu` ForPC MultiUseEntries self))
  (`|ExecutionSequence`
    (:`then_0`
      (`/Game/Mods/StructuresPlusMod/_Scripts/MultiUseMenuFunctions.SP_Add_Internal_Plumbing_Menu_Entries` _entriesout ForPC self))
    (:`then_1`
      (bind _returnvalue (`self.AllowStructureAccess` ForPC))
      (if _returnvalue
        (`KismetArrayLibrary.Array_Add` _entriesout (make `Actor.MultiUseEntry` :`UseString` (select `int` (`self.ForcefieldSetting`) :`0` "Allow Allies" :`1` "Allow None" :`2` "Allow Tribe Only") :`UseIndex` 9003 :`Priority` -1010))
        (`KismetArrayLibrary.Array_Add` _entriesout (make `Actor.MultiUseEntry` :`UseString` (`KismetStringLibrary.Concat_StrStr` "Current Setting: " (select `int` (`self.ForcefieldSetting`) :`0` "Allow Tribe Only" :`1` "Allow Allies" :`2` "Allow None")) :`UseIndex` 9002 :`Priority` -1011 :`bDisableUse` true :`DisableUseColor` (make `Object.Color` 175 255 0 255)))))
    (:`then_2`
      (return _entriesout))))

(fn `BPRefreshedStructureColors`
  (bind _returnvalue (`self.GetStructureColor` 0))
  (`MaterialInstanceDynamic.SetVectorParameterValue` (`self.ForcefieldMat`) "Color0" _returnvalue))

(fn `BPTryMultiUse`
  (params (ForPC :type "PlayerController Object Reference") (UseIndex :type Integer))
  (returns (ReturnValue :type Boolean))
  (`/Game/Mods/StructuresPlusMod/_Scripts/MultiUseMenuFunctions.SP_HandleCommonMultiUseEntries` ForPC UseIndex self false false true)
  (`|ExecutionSequence`
    (:`then_0`
      (switch `int` UseIndex
        (:`9003`
          (bind _nextsetting (`/Game/Mods/StructuresPlusMod/_Scripts/ForcefieldFunctions.SP_GetNextForcefieldSetting` (`self.ForcefieldSetting`)))
          (set `self.ForcefieldSetting` _nextsetting true))))
    (:`then_1`
      (return false))))

(fn `UserConstructionScript`
  (`parent.UserConstructionScript`)
  (if (not (`self.bIsPreviewStructure`))
    (`/Engine/EditorBlueprintResources/ActorMacros.SwitchNetAuthority`
      (:`PlayerServer`
        _)
      (:`Client`
        _))
    (bind _returnvalue (`KismetMaterialLibrary.CreateDynamicMaterialInstance` "/Game/PrimalEarth/StructuresPlus/_Materials/ForceField_MIC.ForceField_MIC"))
    (set `self.ForcefieldMat` _returnvalue)
    (`PrimitiveComponent.SetMaterial` (`self.MyStaticMesh`) 0 (`self.ForcefieldMat`))))