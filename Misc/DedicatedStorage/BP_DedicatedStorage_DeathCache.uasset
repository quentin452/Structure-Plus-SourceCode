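; ARK dedicated-storage death cache holding a count of one resource class, drawn on the HUD, that destroys itself shortly after the count hits zero.
; A "Withdraw Stack" wheel entry moves up to one stack, limited by player capacity and stock, into the player's inventory via S+ helpers.
; BPGetExtraSpecialBlueprintInt doubles as the count adjuster and empty check, while the quantity override reports stock capped at the transfer limit.
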(event Custom|HandleSuicideEvent
  (Utilities|FlowControl|Delay 0.2)
  (Actor|DestroyActor))

(fn ConstructionScript
  (|CallParentFunction))

(fn BPGetMultiUseEntries
  (params (ForPC :type Player%20Controller%20Object%20Reference) (MultiUseEntries :type Array%20of%20Multi%20Use%20Entry%20Structures))
  (bind _entriesout (CallFunction|SPUpdateMultiUseMenu ForPC MultiUseEntries self false false false false))
  (Utilities|FlowControl|Sequence
    (:then_0
      (if (> (Variables|Default|GetResourceCount) 0)
        (Utilities|Array|Add _entriesout (Utilities|Struct|MakeMultiUseEntry "Withdraw Stack" 9001 1500 true))))
    (:then_1
      (return _entriesout))))

(fn BPTryMultiUse
  (params (ForPC :type Player%20Controller%20Object%20Reference) (UseIndex :type Integer))
  (Utilities|FlowControl|Sequence
    (:then_0
      (switch int UseIndex
        (:9001
          (CallFunction|HandleWithdraw ForPC))))
    (:then_1
      (return false))))

(fn ReceiveBeginPlay
  (|CallParentFunction)
  (if (Variables|Default|GetbIsPreviewStructure)
    _))

(fn HandleWithdraw
  (params (PC :type Player%20Controller%20Object%20Reference))
  (bind _resourcecount (Variables|Default|GetResourceCount))
  (bind _selectedresourceclass (Variables|Default|GetSelectedResourceClass))
  (bind _asshooterplayercontroller (Utilities|Casting|CastToShooterPlayerController PC))
  (if (!= _selectedresourceclass 0)
    (bind _outitem (CallFunction|SPGetRemappedItem _selectedresourceclass))
    (bind _returnvalue (Class|VictoryCore|GetClassDefaultObject _outitem))
    (bind _asprimalitem (Utilities|Casting|CastToPrimalItem _returnvalue))
    (LocalVariables|SetStackSize_HW (CallFunction|SPGetItemStackSize _asprimalitem (Game|GetGameMode)))
    (bind _total (CallFunction|SPGetCapacityforItem _outitem (Class|ShooterPlayerController|GetPlayerCharacter _asshooterplayercontroller)))
    (LocalVariables|SetAmtRemoved_HW (Math|Integer|Min(Integer) _total (LocalVariables|GetStackSize_HW) _resourcecount))
    (if (> (LocalVariables|GetAmtRemoved_HW) 0)
      (Utilities|FlowControl|Sequence
        (:then_0
          (bind _qtyremoved (CallFunction|SPRemovefromInventory _outitem (Variables|Default|GetMyInventoryComponent) (LocalVariables|GetAmtRemoved_HW) true false))
          (LocalVariables|SetAmtRemoved_HW _qtyremoved))
        (:then_1
          (if (> (LocalVariables|GetAmtRemoved_HW) 0)
            (if (== (LocalVariables|GetStackSize_HW) 1)
              (CallFunction|SPFastGiveItem (Variables|/Script/ShooterGame.PrimalCharacter|GetMyInventoryComponent (Class|ShooterPlayerController|GetPlayerCharacter _asshooterplayercontroller)) _outitem (LocalVariables|GetAmtRemoved_HW))
              (else
                (Class|PrimalInventoryComponent|BPIncrementItemTemplateQuantity (Variables|/Script/ShooterGame.PrimalCharacter|GetMyInventoryComponent (Class|ShooterPlayerController|GetPlayerCharacter _asshooterplayercontroller)) _outitem (LocalVariables|GetAmtRemoved_HW) true false true false false false 0 false))))))
      (elif (> _resourcecount 0)
        (Class|StructuresPlus|SPMessageClient PC "Inventory limit reached." "Error")))))

(fn BPGetExtraSpecialBlueprintInt
  (params (toCheck :type Integer))
  (Utilities|FlowControl|Sequence
    (:then_0
      (if (== toCheck 0)
        (LocalVariables|SetRetVal_ESB 0)
        (else
          (Variables|Default|SetResourceCount (Math|Integer|Clamp(Integer) (+ (Variables|Default|GetResourceCount) toCheck) 0 (Class|KismetSystemLibrary|MakeLiteralInteger 2147483647)) true)
          (LocalVariables|SetRetVal_ESB (Variables|Default|GetResourceCount)))))
    (:then_1
      (if (<= (Variables|Default|GetResourceCount) 0)
        (CallFunction|HandleSuicideEvent)))
    (:then_2
      (return (LocalVariables|GetRetVal_ESB)))))

(fn BPGetQuantityOfItemWithoutCheckingInventory
  (params (ItemToCheckFor :type Primal%20Item%20Class%20Reference))
  (bind _outitem (CallFunction|SPGetRemappedItem (Variables|Default|GetSelectedResourceClass)))
  (return (Math|Integer|SelectInt (Math|Integer|Min(Integer) (Variables|Default|GetResourceCount) (Variables|Default|GetMaxTransferAmt)) -1 (Utilities|ClassIsChildOf _outitem ItemToCheckFor))))

(fn BPIsValidWaterSourceforPipe
  (params (ForWaterPipe :type Primal%20Structure%20Water%20Pipe%20Object%20Reference))
  (return (not (Utilities|IsValid ForWaterPipe))))

(fn BlueprintDrawHUD
  (params (HUD :type Shooter%20HUD%20Object%20Reference) (CenterX :type Float%20%28single-precision%29) (CenterY :type Float%20%28single-precision%29))
  (bind _selectedresourceclass (Variables|Default|GetSelectedResourceClass))
  (bind _canvas (Variables|/Script/Engine.HUD|GetCanvas HUD))
  (if (!= _selectedresourceclass 0)
    (bind _descriptivename (CallFunction|SPGetDescriptiveName _selectedresourceclass))
    (Class|Canvas|SetDrawColor _canvas (Math|Color|MakeColor 255 225 200 255))
    (Class|Canvas|BPDrawTextCentered _canvas (Variables|/Script/ShooterGame.ShooterHUD|GetNormalFont HUD) (Utilities|String|ToString(Text) (Utilities|Text|FormatText "{resName} : {count}" (Utilities|Text|ToText(String) _descriptivename) (Utilities|Text|ToText(Integer) (Variables|Default|GetResourceCount)))) CenterX (- CenterY 1e+02) 0.8 0.8 true true)))