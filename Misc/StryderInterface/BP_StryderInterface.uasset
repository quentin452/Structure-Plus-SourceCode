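; Structures Plus dino saddle structure (Dedicated Storage Interface) that, while activated, empties chosen items from the dino's inventory.
; Inventory additions trigger a delayed, rate-limited pass that deletes Destroy List items, then bulk-transfers Upload List items to matching team dedicated storages found via custom actor lists.
; Players edit both lists through a buff-driven UI, saved via net exec commands.
; Placement enforces one per saddle, tribe limits and config-driven dino whitelist or blacklist.
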(event Custom|OnInventoryItemAdded_Event
  (params (Inventory :type Primal%20Inventory%20Component%20Object%20Reference) (Item :type Primal%20Item%20Object%20Reference) (AmountAdded :type Integer) (bEquippedItem :type Boolean))
  (Utilities|Time|SetTimerbyFunctionName 0 "TryUpload" 2.0))

(event Custom|HandleBeginPlayEvent
  (bind _linkedstructures (Variables|Default|GetLinkedStructures))
  (Utilities|FlowControl|Delay 1.0)
  (Utilities|FlowControl|Sequence
    (:then_0
      (for _array_element _linkedstructures
        (switch name (Variables|/Script/ShooterGame.PrimalStructure|GetStructureTag _array_element)
          (:SPlus_DedicatedStorage
            _)
          (:SPlus_Storage_Tek
            _))
        (Utilities|Array|Clear (Variables|/Script/ShooterGame.PrimalStructure|GetLinkedStructures _array_element)))
      (Utilities|Array|Clear _linkedstructures))
    (:then_1
      (if (> (Variables|Default|GetTribeLimit) 0)
        (CallFunction|SPAddtoCustomActorList self (Utilities|String|BuildString(Integer) "SPlusDediInterfaces_" "" (Variables|Default|GetTargetingTeam)))))
    (:then_2
      (Variables|Default|SetOnDino (Variables|Default|GetSaddleDino))
      (Utilities|IsValid (Variables|Default|GetOnDino)
        (:Is%20Valid
          (Variables|/Script/ShooterGame.PrimalInventoryComponent|SetbBPNotifyItemAdded (Variables|/Script/ShooterGame.PrimalCharacter|GetMyInventoryComponent (Variables|Default|GetOnDino)) true)
          (EventDispatchers|BindEventtoOnInventoryItemAdded (Variables|/Script/ShooterGame.PrimalCharacter|GetMyInventoryComponent (Variables|Default|GetOnDino)) (delegate Custom|OnInventoryItemAdded_Event)))))))

(event EventEndPlay
  (params (EndPlayReason :type EEndPlayReason%20Enum :default "ActorDestroyed"))
  (bind _ondino (Variables|Default|GetOnDino))
  (Networking|SwitchHasAuthority
    (:Authority
      (if (not (Variables|Default|GetbIsPreviewStructure))
        (switch Utilities|FlowControl|Switch|SwitchonEEndPlayReason EndPlayReason
          (:ActorDestroyed
            (Utilities|FlowControl|Sequence
              (:then_0
                (Utilities|IsValid _ondino
                  (:Is%20Valid
                    (EventDispatchers|UnbindEventfromOnInventoryItemAdded (Variables|/Script/ShooterGame.PrimalCharacter|GetMyInventoryComponent _ondino) (delegate Custom|OnInventoryItemAdded_Event)))))
              (:then_1
                (if (> (Variables|Default|GetTribeLimit) 0)
                  (CallFunction|SPRemovefromCustomActorList self (Utilities|String|BuildString(Integer) "SPlusDediInterfaces_" "" (Variables|Default|GetTargetingTeam))))))))))))

(fn ConstructionScript
  (|CallParentFunction)
  (if (not (Variables|Default|GetbIsPreviewStructure))
    (Class|KismetSystemLibrary|CanRunCosmeticEvents
      (:Yes
        (Rendering|Material|SetMaterial (Variables|Default|GetMyStaticMesh) 0 "/Game/Genesis2/CoreMaterials/MasterMaterials/MIC/MI_Tek_Circuitry.MI_Tek_Circuitry")
        (bind _returnvalue (Rendering|Material|CreateDynamicMaterialInstance "/Game/PrimalEarth/TekTier/Underwater_Cube/Underwater_Cube_Combo_Colorize_MIC.Underwater_Cube_Combo_Colorize_MIC" :!class /Script/Engine.KismetMaterialLibrary))
        (Rendering|Material|SetScalarParameterValue _returnvalue "Top" 1.0 :!class /Script/Engine.MaterialInstanceDynamic)
        (Rendering|Material|SetMaterial (Variables|Default|GetTopMesh) 0 _returnvalue)
        (Rendering|Material|SetMaterial (Variables|Default|GetBottomMesh) 0 _returnvalue)))))

(fn ReceiveBeginPlay
  (bind _returnvalue (Game|GetGameMode))
  (|CallParentFunction)
  (if (not (Variables|Default|GetbIsPreviewStructure))
    (Networking|SwitchHasAuthority
      (:Authority
        (Utilities|FlowControl|Sequence
          (:then_0
            (bind _value (CallFunction|SPGetConfig-Int _returnvalue "TribeInterfaceLimit" 0 0 999999))
            (Variables|Default|SetTribeLimit _value))
          (:then_1
            (bind _value_2 (CallFunction|SPGetConfig-Float _returnvalue "DediInterfaceMinUploadInterval" 1e+01 1.0 999999.0))
            (Variables|Default|SetMinUploadInterval _value_2))
          (:then_2
            (CallFunction|HandleBeginPlayEvent)))))))

(fn BPGetMultiUseEntries
  (params (ForPC :type Player%20Controller%20Object%20Reference) (MultiUseEntries :type Array%20of%20Multi%20Use%20Entry%20Structures))
  (bind _color (CallFunction|SPGetMultiUseSpecialColor))
  (bind _returnvalue (Math|Conversions|ToColor(LinearColor) _color))
  (bind _entriesout (CallFunction|SPUpdateMultiUseMenu ForPC MultiUseEntries self false false false false))
  (Utilities|FlowControl|Sequence
    (:then_0
      (bind _returnvalue_2 (Class|PrimalStructure|AllowStructureAccess ForPC))
      (if _returnvalue_2
        (Utilities|Array|Add _entriesout (Utilities|Struct|MakeMultiUseEntry (Utilities|String|SelectString "Deactivate" "Activate" (Variables|Default|GetIsUploading)) 9000 10000))
        (Utilities|Array|Add _entriesout (Utilities|Struct|MakeMultiUseEntry "[Upload List]" 9001 5000 true _returnvalue))
        (Utilities|Array|Add _entriesout (Utilities|Struct|MakeMultiUseEntry "[Destroy List]" 9002 -5000 true _returnvalue))))
    (:then_1
      (return _entriesout))))

(fn BPTryMultiUse
  (params (ForPC :type Player%20Controller%20Object%20Reference) (UseIndex :type Integer))
  (bind _self self)
  (Utilities|FlowControl|Sequence
    (:then_0
      (bind _asprimalcharacter (Utilities|Casting|CastToPrimalCharacter (Pawn|GetControlledPawn ForPC)))
      (switch int UseIndex
        (:9000
          (Variables|Default|SetIsUploading (not (Variables|Default|GetIsUploading)) true)
          (if (Variables|Default|GetIsUploading)
            (CallFunction|TryUpload)))
        (:9001
          (bind _returnvalue (Class|PrimalBuff|StaticAddBuff "/Game/Mods/StructuresPlusMod/_Buffs/Buff_StructuresPlus_StryderInterface.Buff_StructuresPlus_StryderInterface_C" _asprimalcharacter 0 0 false))
          (bind _asbuff_structuresplus_stryderinterface_c (Utilities|Casting|CastToBuff_StructuresPlus_StryderInterface _returnvalue))
          (Default|InitializeUI _asbuff_structuresplus_stryderinterface_c _self true (CallFunction|GetPullList false) (Variables|Default|GetUploadList)))
        (:9002
          (bind _returnvalue_2 (Class|PrimalBuff|StaticAddBuff "/Game/Mods/StructuresPlusMod/_Buffs/Buff_StructuresPlus_StryderInterface.Buff_StructuresPlus_StryderInterface_C" _asprimalcharacter 0 0 false))
          (bind _asbuff_structuresplus_stryderinterface_c_2 (Utilities|Casting|CastToBuff_StructuresPlus_StryderInterface _returnvalue_2))
          (Default|InitializeUI _asbuff_structuresplus_stryderinterface_c_2 _self false (CallFunction|GetPullList true) (Variables|Default|GetDestroyList)))))
    (:then_1
      (return true))))

(fn TryUpload
  (bind _returnvalue (Utilities|Time|GetGameTimeinSeconds))
  (if (and (Variables|Default|GetIsUploading) (> _returnvalue (Variables|Default|GetNextUploadTime)))
    (Variables|Default|SetNextUploadTime (+ _returnvalue (Variables|Default|GetMinUploadInterval)))
    (Utilities|IsValid (Variables|Default|GetOnDino)
      (:Is%20Valid
        (CallFunction|ProcessDestruction)
        (CallFunction|ProcessUpload)))))

(fn BPIsAllowedtoBuildEx
  (params (OutPlacementData :type Placement%20Data%20Structure%20%28by%20ref%29) (CurrentAllowedReason :type Integer) (PC :type Player%20Controller%20Object%20Reference) (bFinalPlacement :type Boolean) (bChoosingRotation :type Boolean))
  (bind _dinocharacter (Utilities|Struct|BreakPlacementData OutPlacementData))
  (bind _myinventorycomponent (Variables|/Script/ShooterGame.PrimalCharacter|GetMyInventoryComponent _dinocharacter))
  (LocalVariables|SetBuildReason_IAB CurrentAllowedReason)
  (Utilities|FlowControl|Sequence
    (:then_0
      (if (>= CurrentAllowedReason 0)
        (LocalVariables|SetBuildReason_IAB -17)
        (Utilities|IsValid _dinocharacter
          (:Is%20Valid
            (if (== (Variables|/Script/Engine.Actor|GetTargetingTeam _dinocharacter) (Variables|Default|GetTargetingTeam))
              (Utilities|IsValid _myinventorycomponent
                (:Is%20Valid
                  (bind _returnvalue (Class|PrimalInventoryComponent|GetEquippedItemOfType _myinventorycomponent "DinoSaddle"))
                  (if (or (Utilities|IsValid _returnvalue) (Utilities|ClassIsChildOf (Utilities|GetClass _dinocharacter) "/Game/Genesis2/Dinos/TekStrider/TekStrider_Character_BP.TekStrider_Character_BP_C"))
                    (LocalVariables|SetBuildReason_IAB 1)
                    (if bFinalPlacement
                      (Networking|SwitchHasAuthority
                        (:Authority
                          (bind _array_element (Utilities|Array|ForEachLoopwithBreak (Variables|/Script/ShooterGame.PrimalDinoCharacter|GetSaddleStructures _dinocharacter) :!label _label)
                            (:LoopBody
                              (Utilities|IsValid (Utilities|Struct|BreakPrimalSaddleStructure _array_element)
                                (:Is%20Valid
                                  (if (== (Utilities|GetClass (Utilities|Struct|BreakPrimalSaddleStructure _array_element)) "BP_StryderInterface_C")
                                    (LocalVariables|SetFoundAnotherInterface_IAB true)
                                    (goto _label Break)))))
                            (:Completed
                              (if (LocalVariables|GetFoundAnotherInterface_IAB)
                                (LocalVariables|SetBuildReason_IAB -899)
                                (Class|StructuresPlus|SPMessageClient PC "Can only place 1 interface on a saddle." "Error")))))))))))))))
    (:then_1
      (bind _buildreason (CallFunction|SPCheckTribeLimit self "Dedicated Storage Interface" (LocalVariables|GetBuildReason_IAB) (Variables|Default|GetTribeLimit) (Utilities|String|BuildString(Integer) "SPlusDediInterfaces_" "" (Variables|Default|GetTargetingTeam)) bFinalPlacement PC))
      (bind _newreason (CallFunction|CheckAgainstLists _buildreason OutPlacementData PC bFinalPlacement))
      (return _newreason))))

(fn BPOverrideCantBuildReasonString
  (params (CantBuildReason :type Integer))
  (Utilities|FlowControl|Sequence
    (:then_0
      (if (== CantBuildReason -699)
        (LocalVariables|SetStringOverride_BRS "You have reached your tribe limit for interfaces.")
        (elif (== CantBuildReason -799)
          (LocalVariables|SetStringOverride_BRS "Your server admin has disabled placement on this dino.")
          (elif (== CantBuildReason -899)
            (LocalVariables|SetStringOverride_BRS "Only 1 Interface can be placed on a saddle platform.")))))
    (:then_1
      (return (LocalVariables|GetStringOverride_BRS)))))

(fn BPServerHandleNetExecCommand
  (params (FromPC :type Player%20Controller%20Object%20Reference) (CommandName :type Name :default "None") (ExecParams :type BP%20Net%20Exec%20Params%20Structure%20%28by%20ref%29))
  (bind _temparray_hne (LocalVariables|GetTempArray_HNE))
  (Utilities|FlowControl|Sequence
    (:then_0
      (bind _assplus_misc_comobject_c (Utilities|Casting|CastToSPlus_Misc_ComObject (Utilities|Struct|BreakBPNetExecParams ExecParams)))
      (for _array_element (Variables|/Game/Mods/StructuresPlusMod/_ComObjects/SPlus_Misc_ComObject.SPlus_Misc_ComObject_C|GetObjectClasses _assplus_misc_comobject_c)
        (bind _asprimalitem (Utilities|Casting|CastToPrimalItemClass _array_element))
        (Utilities|Array|Add (LocalVariables|GetTempArray_HNE) _asprimalitem))
      (switch name CommandName
        (:SetUploadList
          (Variables|Default|SetUploadList _temparray_hne))
        (:SetDestroyList
          (Variables|Default|SetDestroyList _temparray_hne))))
    (:then_1
      (return true))))

(fn ProcessDestruction
  (bind _ondino (Variables|Default|GetOnDino))
  (bind _myinventorycomponent (Variables|/Script/ShooterGame.PrimalCharacter|GetMyInventoryComponent _ondino))
  (for _array_element (Variables|Default|GetDestroyList)
    (bind _returnvalue (Class|PrimalInventoryComponent|GetItemTemplateQuantity _myinventorycomponent _array_element 0 true false true false))
    (if (> _returnvalue 0)
      (Class|PrimalInventoryComponent|BPIncrementItemTemplateQuantity _myinventorycomponent _array_element (* _returnvalue -1) true false true false false false 0 false))))

(fn ProcessUpload
  (bind _ondino (Variables|Default|GetOnDino))
  (bind _myinventorycomponent (Variables|/Script/ShooterGame.PrimalCharacter|GetMyInventoryComponent _ondino))
  (bind _returnvalue (Class|VictoryCore|GetCustomActorList (Class|Actor|GetWorld) (Utilities|String|StringToName (Utilities|String|BuildString(Integer) "SPlusDedicatedStorage_" "" (Variables|Default|GetTargetingTeam)))))
  (Utilities|IsValid _returnvalue
    (:Is%20Valid
      (LocalVariables|SetDoEverything_PU (Utilities|Array|ContainsItem (Variables|Default|GetUploadList) (Variables|Default|GetEverythingClass)))
      (for _array_element (Variables|/Script/ShooterGame.CustomActorList|GetActorList _returnvalue)
        (bind _asprimalstructureitemcontainer (Utilities|Casting|CastToPrimalStructureItemContainer _array_element))
        (if (Utilities|Array|IsValidIndex (Variables|/Script/ShooterGame.PrimalInventoryComponent|GetRemoteAddItemOnlyAllowItemClasses (Variables|/Script/ShooterGame.PrimalStructureItemContainer|GetMyInventoryComponent _asprimalstructureitemcontainer)))
          (if (!= (Utilities|Array|Get(acopy) (Variables|/Script/ShooterGame.PrimalInventoryComponent|GetRemoteAddItemOnlyAllowItemClasses (Variables|/Script/ShooterGame.PrimalStructureItemContainer|GetMyInventoryComponent _asprimalstructureitemcontainer))) "/Script/ShooterGame.PrimalItem")
            (if (or (LocalVariables|GetDoEverything_PU) (>= (Utilities|Array|FindItem (Variables|Default|GetUploadList) (Utilities|Array|Get(acopy) (Variables|/Script/ShooterGame.PrimalInventoryComponent|GetRemoteAddItemOnlyAllowItemClasses (Variables|/Script/ShooterGame.PrimalStructureItemContainer|GetMyInventoryComponent _asprimalstructureitemcontainer)))) 0))
              (CallFunction|AddtoDediList (Utilities|Array|Get(acopy) (Variables|/Script/ShooterGame.PrimalInventoryComponent|GetRemoteAddItemOnlyAllowItemClasses (Variables|/Script/ShooterGame.PrimalStructureItemContainer|GetMyInventoryComponent _asprimalstructureitemcontainer))) _asprimalstructureitemcontainer (LocalVariables|GetTempDediStorages_PU))))))
      (for _array_element_2 (LocalVariables|GetTempDediStorages_PU)
        (bind _returnvalue_2 (Class|PrimalInventoryComponent|GetItemTemplateQuantity _myinventorycomponent (.ItemClass (Utilities|Struct|BreakSP_DediStorageResult _array_element_2)) 0 true false true false))
        (if (> _returnvalue_2 0)
          (Utilities|Array|Add (LocalVariables|GetDediStorageAlphas_PU) (Utilities|Struct|MakeSP_AlphabetizationObject (.ItemClass (Utilities|Struct|BreakSP_DediStorageResult _array_element_2))))
          (Utilities|Array|AppendArray (LocalVariables|GetDediStorages_PU) (.Structures (Utilities|Struct|BreakSP_DediStorageResult _array_element_2)))))
      (if (and (> (Utilities|Array|Length (LocalVariables|GetDediStorageAlphas_PU)) 0) (> (Utilities|Array|Length (LocalVariables|GetDediStorages_PU)) 0))
        (CallFunction|SPDoBulkTransferEx 0 (Utilities|Struct|MakeSPTransferRequest (Utilities|Array|MakeArray (Utilities|Struct|MakeSP_AlphabetizationObject "/Script/ShooterGame.PrimalStructureItemContainer")) (LocalVariables|GetDediStorageAlphas_PU)) (Utilities|Array|MakeArray _myinventorycomponent) (Utilities|Array|MakeArray) (LocalVariables|GetDediStorages_PU))))))

(fn AddtoDediList
  (params (ItemClass :type Primal%20Item%20Class%20Reference) (DediStorage :type Primal%20Structure%20Item%20Container%20Object%20Reference) (DediStorageList :type Array%20of%20SP%20Dedi%20Storage%20Result%20Structures))
  (LocalVariables|SetFoundIndex_ADL -1)
  (bind (_array_element _array_index) (Utilities|Array|ForEachLoopwithBreak DediStorageList :!label _label)
    (:LoopBody
      (if (== ItemClass (Utilities|Struct|BreakSP_DediStorageResult _array_element))
        (LocalVariables|SetFoundIndex_ADL _array_index)
        (LocalVariables|SetCurDediEntry_ADL _array_element)
        (goto _label Break)))
    (:Completed
      (if (>= (LocalVariables|GetFoundIndex_ADL) 0)
        (LocalVariables|SetNewStructures_ADL (Utilities|Struct|BreakSP_DediStorageResult (LocalVariables|GetCurDediEntry_ADL)))
        (Utilities|Array|Add (LocalVariables|GetNewStructures_ADL) DediStorage)
        (Utilities|Struct|SetmembersinSP_DediStorageResult (LocalVariables|GetCurDediEntry_ADL) (LocalVariables|GetNewStructures_ADL))
        (Utilities|Array|SetArrayElem DediStorageList (LocalVariables|GetFoundIndex_ADL) (LocalVariables|GetCurDediEntry_ADL))
        (else
          (Utilities|Array|Add DediStorageList (Utilities|Struct|MakeSP_DediStorageResult ItemClass (Utilities|Array|MakeArray DediStorage))))))))

(fn GetPullList
  (params (AddSeeds :type Boolean))
  (bind _returnvalue (Game|GetGameMode))
  (Utilities|FlowControl|Sequence
    (:then_0
      (if (== (Utilities|Array|Length (Variables|Default|GetResourceList)) 0)
        (bind _assplusglobalactor_c (Utilities|Casting|CastToSPlusGlobalActor (CallFunction|SPGetGlobalActor self)))
        (Utilities|FlowControl|Sequence
          (:then_0
            (bind _value (CallFunction|SPGetConfig-Bool _returnvalue "DedicatedStorageAllowNonStackables"))
            (if _value
              (Variables|Default|SetResourceList (Variables|/Game/Mods/StructuresPlusMod/SPlusGlobalActor.SPlusGlobalActor_C|GetPullResourceList _assplusglobalactor_c))
              (else
                (Utilities|Array|Clear (Variables|Default|GetResourceList))
                (for _array_element (Variables|/Game/Mods/StructuresPlusMod/SPlusGlobalActor.SPlusGlobalActor_C|GetPullResourceList _assplusglobalactor_c)
                  (bind _returnvalue_2 (Class|VictoryCore|GetClassDefaultObject (Utilities|Struct|BreakSP_AlphabetizationObject _array_element)))
                  (bind _asprimalitem (Utilities|Casting|CastToPrimalItem _returnvalue_2))
                  (if (> (CallFunction|SPGetItemStackSize _asprimalitem _returnvalue) 1)
                    (Utilities|Array|Add (Variables|Default|GetResourceList) _array_element))))))
          (:then_1
            (bind _classarray (CallFunction|SPAlphaObjArraytoClassArray (Variables|Default|GetResourceList)))
            (for _array_element_2 (Variables|Default|GetSeedClasses)
              (bind _outitem (CallFunction|SPGetRemappedItem _array_element_2))
              (if (not (Utilities|Array|ContainsItem _classarray _outitem))
                (Utilities|Array|Add (Variables|Default|GetSeedList) (Utilities|Struct|MakeSP_AlphabetizationObject _outitem))))
            (Utilities|Array|AppendArray (Variables|Default|GetSeedList) (Variables|Default|GetResourceList))))))
    (:then_1
      (return (select AddSeeds (Variables|Default|GetSeedList) (Variables|Default|GetResourceList))))))

(fn CheckAgainstLists
  (params (CurReason :type Integer) (PlacementData :type Placement%20Data%20Structure) (PC :type Player%20Controller%20Object%20Reference) (IsFinal :type Boolean))
  (bind _dinocharacter (Utilities|Struct|BreakPlacementData PlacementData))
  (bind _returnvalue (Game|GetGameMode))
  (bind _returnvalue_2 (Utilities|GetClass _dinocharacter))
  (bind _returnvalue_3 (Utilities|GetClassDisplayName _returnvalue_2))
  (LocalVariables|SetBuildReason_CAL CurReason)
  (Utilities|FlowControl|Sequence
    (:then_0
      (if (and IsFinal (> (LocalVariables|GetBuildReason_CAL) 0))
        (bind _value (CallFunction|SPGetConfig-String _returnvalue "DediInterfaceDinoWhitelist"))
        (if (> (Utilities|String|Len _value) 0)
          (if (< (Utilities|String|FindSubstring _value _returnvalue_3) 0)
            (LocalVariables|SetBuildReason_CAL -799 :!label _label)
            (Class|StructuresPlus|SPMessageClient PC "Your server admin has disabled placement on this dino." "Error"))
          (else
            (bind _value_2 (CallFunction|SPGetConfig-String _returnvalue "DediInterfaceDinoBlacklist"))
            (if (and (> (Utilities|String|Len _value_2) 0) (>= (Utilities|String|FindSubstring _value_2 _returnvalue_3) 0))
              (goto _label))))))
    (:then_1
      (return (LocalVariables|GetBuildReason_CAL)))))