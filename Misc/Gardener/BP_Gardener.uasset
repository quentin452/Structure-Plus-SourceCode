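; Gardener structure, a Structures Plus item collector that periodically gathers from crop plots while activated.
; On server begin play it sets slot count and scan radius (in foundations) from game config and enables crop plot collection.
; A self-rescheduling DoScan timer runs the inherited crop collection.
; Team members edit ignore and destroy lists through an ItemAggregator buff UI, which returns selections via net exec commands.
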(fn `BPGetMultiUseEntries`
  (params (ForPC :type "PlayerController Object Reference") (MultiUseEntries :type "Array of Actor.MultiUseEntry Structure (by ref)"))
  (returns (ReturnValue :type "Array of Actor.MultiUseEntry Structure"))
  (bind _returnvalue (`KismetMathLibrary.Conv_LinearColorToColor` (`/Game/Mods/StructuresPlusMod/_Scripts/MultiUseMenuFunctions.SP_GetMultiUseSpecialColor`)))
  (bind _returnvalue_2 (`parent.BPGetMultiUseEntries` ForPC MultiUseEntries))
  (`|ExecutionSequence`
    (:`then_0`
      (if (== (`Actor.TargetingTeam` ForPC) (`self.TargetingTeam`))
        (`KismetArrayLibrary.Array_Add` _returnvalue_2 (make `Actor.MultiUseEntry` :`UseString` "[View Ignore List]" :`UseIndex` 9004 :`Priority` -450 :`bDisplayOnInventoryUISecondary` true :`bOverrideUseTextColor` true :`UseTextColor` _returnvalue))
        (`KismetArrayLibrary.Array_Add` _returnvalue_2 (make `Actor.MultiUseEntry` :`UseString` "[View Destroy List]" :`UseIndex` 9005 :`Priority` -500 :`bOverrideUseTextColor` true :`bDisplayOnInventoryUITertiary` true :`UseTextColor` _returnvalue))))
    (:`then_1`
      (return _returnvalue_2))))

(fn `BPServerHandleNetExecCommand`
  (params (FromPC :type "PlayerController Object Reference") (CommandName :type Name) (ExecParams :type "Actor.BPNetExecParams Structure (by ref)"))
  (returns (ReturnValue :type Boolean))
  (`|ExecutionSequence`
    (:`then_0`
      (`/Engine/EditorBlueprintResources/StandardMacros.IsValid` FromPC
        (:`Is Valid`
          (bind _assplus_misc_comobject_c (cast `/Game/Mods/StructuresPlusMod/_ComObjects/SPlus_Misc_ComObject` (`.ObjParam1` (break `Actor.BPNetExecParams` ExecParams))))
          (switch `name` CommandName
            (:`GardenerSetBlackList`
              (bind _objectclasses (`/Game/Mods/StructuresPlusMod/_ComObjects/SPlus_Misc_ComObject.ObjectClasses` _assplus_misc_comobject_c))
              (set `self.CollectionBlacklist` _objectclasses))
            (:`GardenerSetDestroyList`
              (set `self.CollectionDestroylist` _objectclasses))))))
    (:`then_1`
      (return true))))

(fn `BPTryMultiUse`
  (params (ForPC :type "PlayerController Object Reference") (UseIndex :type Integer))
  (returns (ReturnValue :type Boolean))
  (`parent.BPTryMultiUse` ForPC UseIndex)
  (`|ExecutionSequence`
    (:`then_0`
      (switch `int` UseIndex
        (:`9004`
          (bind _asshooterplayercontroller (cast `ShooterPlayerController` ForPC))
          (bind _returnvalue (`PrimalBuff.StaticAddBuff` "/Game/Mods/StructuresPlusMod/_Buffs/Buff_StructuresPlus_ItemAggregator.Buff_StructuresPlus_ItemAggregator_C" (`ShooterPlayerController.GetPlayerCharacter` _asshooterplayercontroller)))
          (bind _asbuff_structuresplus_itemaggregator_c (cast `/Game/Mods/StructuresPlusMod/_Buffs/Buff_StructuresPlus_ItemAggregator` _returnvalue))
          (`/Game/Mods/StructuresPlusMod/_Buffs/Buff_StructuresPlus_ItemAggregator.InitializeUI_-_SelectList` _asbuff_structuresplus_itemaggregator_c "Items to Ignore" "GardenerSetBlackList" self (`self.CollectionBlacklist`)))
        (:`9005`
          (bind _asshooterplayercontroller_2 (cast `ShooterPlayerController` ForPC))
          (bind _returnvalue_2 (`PrimalBuff.StaticAddBuff` "/Game/Mods/StructuresPlusMod/_Buffs/Buff_StructuresPlus_ItemAggregator.Buff_StructuresPlus_ItemAggregator_C" (`ShooterPlayerController.GetPlayerCharacter` _asshooterplayercontroller_2)))
          (bind _asbuff_structuresplus_itemaggregator_c_2 (cast `/Game/Mods/StructuresPlusMod/_Buffs/Buff_StructuresPlus_ItemAggregator` _returnvalue_2))
          (`/Game/Mods/StructuresPlusMod/_Buffs/Buff_StructuresPlus_ItemAggregator.InitializeUI_-_SelectList` _asbuff_structuresplus_itemaggregator_c_2 "Items to Destroy" "GardenerSetDestroyList" self (`self.CollectionDestroylist`)))))
    (:`then_1`
      (return true))))

(fn `DoScan`
  (if (`self.bContainerActivated`)
    (`PrimalInventoryComponent.InventoryRefresh` (`self.MyInventoryComponent`))
    (`self.Collect_-_Crops`)
    (`KismetSystemLibrary.K2_SetTimer` null "DoScan" (`self.GetScanInterval`))))

(fn `ReceiveBeginPlay`
  (bind _returnvalue (`GameplayStatics.GetGameMode`))
  (`parent.ReceiveBeginPlay`)
  (if (not (`self.bIsPreviewStructure`))
    (`/Engine/EditorBlueprintResources/ActorMacros.Switch Has Authority`
      (:`Authority`
        (`|ExecutionSequence`
          (:`then_0`
            (bind _value (`/Game/Mods/StructuresPlusMod/_Scripts/ConfigFunctions.SP_GetConfigSetting_-_InventorySize` _returnvalue "GardenerSlotCount" 300))
            (set `self.InvSlotOverride` _value true))
          (:`then_1`
            (bind _value_2 (`/Game/Mods/StructuresPlusMod/_Scripts/ConfigFunctions.SP_GetConfig_-_Int` _returnvalue "GardenerRangeInFoundations" 25 1 100))
            (set `self.ScanRadius` (* _value_2 300.0) true))
          (:`then_2`
            (setmembers `/Game/Mods/StructuresPlusMod/_Structs/SP_ItemCollectorCollectData` :`StructRef` (`self.CollectData_Ground`) :`CropPlots` true)))))))

(fn `UserConstructionScript`
  (`parent.UserConstructionScript`))