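; Metal elevator track structure that lets same-team players add stops to its elevator platform through an "Add Stop" multi-use entry.
; It finds the platform with a capped search through linked track pieces.
; A stop's height derives from the track mesh's top, is rejected if duplicate or over the limit, then gets sorted, multicast to the platform and confirmed by notification.
; The placement check also overrides one specific build-refusal code.
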(fn ConstructionScript
  (|CallParentFunction))

(fn BPIsAllowedtoBuild
  (params (OutPlacementData :type Placement%20Data%20Structure%20%28by%20ref%29) (CurrentAllowedReason :type Integer))
  (return (Math|Integer|SelectInt 1 CurrentAllowedReason (== CurrentAllowedReason -9))))

(fn BPGetMultiUseEntries
  (params (ForPC :type Player%20Controller%20Object%20Reference) (MultiUseEntries :type Array%20of%20Multi%20Use%20Entry%20Structures))
  (bind _entriesout (CallFunction|SPUpdateMultiUseMenu ForPC MultiUseEntries self false false false false))
  (Utilities|FlowControl|Sequence
    (:then_0
      (if (== (Variables|/Script/Engine.Actor|GetTargetingTeam ForPC) (Variables|Default|GetTargetingTeam))
        (Utilities|Array|Add _entriesout (Utilities|Struct|MakeMultiUseEntry "Add Stop" 9001 -1001 false))))
    (:then_1
      (return _entriesout))))

(fn BPTryMultiUse
  (params (ForPC :type Player%20Controller%20Object%20Reference) (UseIndex :type Integer))
  (Utilities|FlowControl|Sequence
    (:then_0
      (switch int UseIndex
        (:9001
          (bind _elevator (CallFunction|GetAttachedPlatform))
          (CallFunction|SetStop ForPC _elevator))))
    (:then_1
      (return true))))

(fn GetAttachedPlatform
  (LocalVariables|SetSelfObj self)
  (Utilities|Array|Add (LocalVariables|GetUnprocessed) (LocalVariables|GetSelfObj))
  (while (Math|Boolean|ANDBoolean (> (Utilities|Array|Length (LocalVariables|GetUnprocessed)) 0) (< (LocalVariables|GetCounter) 500) (not (Utilities|IsValid (LocalVariables|GetPlatform))))
    (LocalVariables|SetCounter (+ (LocalVariables|GetCounter) 1))
    (bind _array_element (Utilities|Array|ForEachLoopwithBreak (LocalVariables|GetUnprocessed) :!label _label)
      (:LoopBody
        (bind _array_element_2 (Utilities|Array|ForEachLoopwithBreak (Variables|/Script/ShooterGame.PrimalStructure|GetLinkedStructures _array_element) :!label _label_2)
          (:LoopBody
            (bind _asbase_elevatorplatform_c (Utilities|Casting|CastToBase_ElevatorPlatform _array_element_2)
              (:then
                (LocalVariables|SetPlatform _asbase_elevatorplatform_c)
                (goto _label_2 Break))
              (:CastFailed
                (bind _asbp_elevatortrack_metal_c (Utilities|Casting|CastToBP_ElevatorTrack_Metal _array_element_2))
                (if (not (or (Utilities|Array|ContainsItem (LocalVariables|GetUnprocessed) _asbp_elevatortrack_metal_c) (Utilities|Array|ContainsItem (LocalVariables|GetProcessed) _asbp_elevatortrack_metal_c)))
                  (Utilities|Array|Add (LocalVariables|GetUnprocessed) _asbp_elevatortrack_metal_c)))))
          (:Completed
            (Utilities|IsValid (LocalVariables|GetPlatform)
              (:Is%20Valid
                (goto _label Break))
              (:Is%20Not%20Valid
                (Utilities|Array|RemoveItem (LocalVariables|GetUnprocessed) _array_element)
                (Utilities|Array|Add (LocalVariables|GetProcessed) _array_element))))))))
  (return (LocalVariables|GetPlatform)))

(fn SetStop
  (params (PC :type Player%20Controller%20Object%20Reference) (Elevator :type Base%20Elevator%20Platform%20Object%20Reference))
  (bind _mystaticmesh (Variables|Default|GetMyStaticMesh))
  (bind (_origin _boxextent) (Collision|GetComponentBounds _mystaticmesh))
  (bind _returnvalue (+ (.z _origin) (.z _boxextent)))
  (bind _returnvalue_2 (- _returnvalue 35.0))
  (bind _asshooterplayercontroller (Utilities|Casting|CastToShooterPlayerController PC))
  (Utilities|IsValid Elevator
    (:Is%20Valid
      (if (Utilities|Array|ContainsItem (Variables|/Game/Mods/StructuresPlusMod/Misc/Elevators/Platforms/Base_ElevatorPlatform.Base_ElevatorPlatform_C|GetStops Elevator) _returnvalue_2)
        (Class|ShooterPlayerController|ClientServerNotification _asshooterplayercontroller "Stop exists." "(R=1.000000,G=0.000000,B=0.000000,A=1.000000)" 1.25 3.0)
        (elif (>= (Utilities|Array|Length (Variables|/Game/Mods/StructuresPlusMod/Misc/Elevators/Platforms/Base_ElevatorPlatform.Base_ElevatorPlatform_C|GetStops Elevator)) 8)
          (Class|ShooterPlayerController|ClientServerNotification _asshooterplayercontroller "Max number of stops reached." "(R=0.980000,G=0.019600,B=0.019600,A=1.000000)" 1.25 3.0)
          (else
            (Utilities|Array|Add (Variables|/Game/Mods/StructuresPlusMod/Misc/Elevators/Platforms/Base_ElevatorPlatform.Base_ElevatorPlatform_C|GetStops Elevator) _returnvalue_2)
            (bind _arrayout (CallFunction|SPSortArrayASC (Variables|/Game/Mods/StructuresPlusMod/Misc/Elevators/Platforms/Base_ElevatorPlatform.Base_ElevatorPlatform_C|GetStops Elevator)))
            (Variables|/Game/Mods/StructuresPlusMod/Misc/Elevators/Platforms/Base_ElevatorPlatform.Base_ElevatorPlatform_C|SetStops Elevator _arrayout false)
            (Class|Actor|MulticastProperty Elevator "Stops")
            (Default|UpdateStopsEvent Elevator (Variables|/Game/Mods/StructuresPlusMod/Misc/Elevators/Platforms/Base_ElevatorPlatform.Base_ElevatorPlatform_C|GetStops Elevator))
            (Class|ShooterPlayerController|ClientServerNotification _asshooterplayercontroller "Stop added." "(R=0.000000,G=0.166448,B=1.000000,A=1.000000)" 1.25 3.0)))))
    (:Is%20Not%20Valid
      (Class|ShooterPlayerController|ClientServerNotification _asshooterplayercontroller "Add platform before adding stops." "(R=0.995000,G=0.019900,B=0.019900,A=1.000000)" 1.25 3.0))))

(fn ReceiveBeginPlay
  (|CallParentFunction)
  (if (not (Variables|Default|GetbIsPreviewStructure))
    (Networking|SwitchHasAuthority)))