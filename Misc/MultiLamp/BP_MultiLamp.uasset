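; BP_MultiLamp is a placeable lamp structure with configurable color, intensity and automatic day/night switching, editable by same-team players through a multi-tool buff.
; Settings drive the emitter child actor's point light and particle color, plus a dynamic emissive material.
; Authority-started timers blink or ping-pong blend between primary and secondary colors.
; A looping CheckTime timer switches the lamp on at night, respecting manual toggles until the next day/night change.
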(event Custom|SetLightingEvent
  (params (Settings :type SP%20Light%20Settings%20Structure))
  (Variables|Default|SetLightSettings Settings false)
  (CallFunction|HandlePrimaryColor)
  (Networking|SwitchHasAuthority
    (:Authority
      (CallFunction|HandleStartInterval)
      (if (Utilities|Struct|BreakSPLightSettings Settings)
        (Variables|Default|SetManualActivationState 0)
        (Utilities|Time|SetTimerbyFunctionName 0 "CheckTime" 1e+01 true)
        (else
          (Utilities|Time|ClearTimerbyFunctionName 0 "CheckTime"))))))

(event Custom|HandleBeginPlayEvent
  (Utilities|FlowControl|Delay 2.0)
  (Utilities|FlowControl|Sequence
    (:then_0
      (if (Utilities|Struct|BreakSPLightSettings (Variables|Default|GetLightSettings))
        (Utilities|Time|SetTimerbyFunctionName 0 "CheckTime" 1e+01 true)))
    (:then_1
      (CallFunction|HandleStartInterval))))

(event Custom|HandleIntervalLightEvent
  (Utilities|FlowControl|Sequence
    (:then_0
      (if (.doblink (Variables|Default|GetLightSettings))
        (Variables|Default|SetLerpValue (Math|Float|SelectFloat 1.0 0.0 (== (Variables|Default|GetLerpValue) 0.0)))
        (else
          (Variables|Default|SetLerpValue (+ (Variables|Default|GetLerpValue) (* (Variables|Default|GetLerpIncrement) (Variables|Default|GetLerpMultiplier))))
          (if (<= (Variables|Default|GetLerpValue) 0.0)
            (Variables|Default|SetLerpMultiplier 1.0)
            (elif (>= (Variables|Default|GetLerpValue) 1.0)
              (Variables|Default|SetLerpMultiplier -1.0))))))
    (:then_1
      (CallFunction|IntervalLightEvent (Variables|Default|GetLerpValue)))))

(event Custom|IntervalLightEvent
  (params (CurrentLerp :type Float%20%28single-precision%29))
  (bind _lightsettings (Variables|Default|GetLightSettings))
  (bind _returnvalue (Math|Float|Lerp (.a (.primarycolor _lightsettings)) (.a (.secondarycolor _lightsettings)) CurrentLerp))
  (bind _returnvalue_2 (Math|Color|Lerp(LinearColor) (Utilities|Struct|MakeLinearColor (.r (.primarycolor _lightsettings)) (.g (.primarycolor _lightsettings)) (.b (.primarycolor _lightsettings)) 1.0) (Utilities|Struct|MakeLinearColor (.r (.secondarycolor _lightsettings)) (.g (.secondarycolor _lightsettings)) (.b (.secondarycolor _lightsettings)) 1.0) CurrentLerp))
  (bind (_r _g _b) (Utilities|Struct|BreakLinearColor _returnvalue_2))
  (Utilities|SwitchNetAuthority
    (:PlayerServer
      _)
    (:Client
      _))
  (bind _aslamppostemitteromni_c (Utilities|Casting|CastToLampPostEmitterOmni (Variables|/Script/Engine.ChildActorComponent|GetChildActor (Variables|Default|GetActivatedEmitter))))
  (Rendering|Components|Light|SetLightColor (Variables|/Game/PrimalEarth/Test/LampPostEmitterOmni.LampPostEmitterOmni_C|GetPointLight1 _aslamppostemitteromni_c) (Utilities|Struct|MakeLinearColor _r _g _b 1.0))
  (Rendering|Components|Light|SetIntensity (Variables|/Game/PrimalEarth/Test/LampPostEmitterOmni.LampPostEmitterOmni_C|GetPointLight1 _aslamppostemitteromni_c) _returnvalue)
  (Effects|Components|ParticleSystem|SetVectorParameter (Variables|/Script/Engine.Emitter|GetParticleSystemComponent _aslamppostemitteromni_c) "LightColor" (Math|Vector|MakeVector _r _g _b))
  (CallFunction|SetActiveMaterialProperties _r _g _b _returnvalue))

(event EventBPContainerDeactivated
  (CallFunction|HandlePrimaryColor)
  (Utilities|Time|ClearTimerbyFunctionName 0 "HandleIntervalLightEvent"))

(event EventBPContainerActivated
  (CallFunction|HandlePrimaryColor)
  (Networking|SwitchHasAuthority
    (:Authority
      (CallFunction|HandleStartInterval))))

(fn ConstructionScript
  (|CallParentFunction))

(fn BPIsAllowedtoBuild
  (params (OutPlacementData :type Placement%20Data%20Structure%20%28by%20ref%29) (CurrentAllowedReason :type Integer))
  (return (Math|Integer|SelectInt 1 CurrentAllowedReason (== CurrentAllowedReason -9))))

(fn BPGetMultiUseEntries
  (params (ForPC :type Player%20Controller%20Object%20Reference) (MultiUseEntries :type Array%20of%20Multi%20Use%20Entry%20Structures))
  (bind _entriesout (CallFunction|SPUpdateMultiUseMenu ForPC MultiUseEntries self false false false false))
  (Utilities|FlowControl|Sequence
    (:then_0
      (if (== (Variables|/Script/Engine.Actor|GetTargetingTeam ForPC) (Variables|Default|GetTargetingTeam))
        (Utilities|Array|Add _entriesout (Utilities|Struct|MakeMultiUseEntry "[Change Settings]" 9001 -10 true (Math|Conversions|ToColor(LinearColor) (CallFunction|SPGetMultiUseSpecialColor))))))
    (:then_1
      (return _entriesout))))

(fn BPTryMultiUse
  (params (ForPC :type Player%20Controller%20Object%20Reference) (UseIndex :type Integer))
  (bind _bcontaineractivated (Variables|Default|GetbContainerActivated))
  (bind _lightsettings (Variables|Default|GetLightSettings))
  (bind (_postdawnoffset _preduskoffset) (Utilities|Struct|BreakSPLightSettings _lightsettings))
  (Utilities|FlowControl|Sequence
    (:then_0
      (if (== UseIndex 9001)
        (CallFunction|SPApplyMultiToolBuff 3 ForPC self)))
    (:then_1
      (if (== UseIndex 600)
        (bind _isday (CallFunction|SPIsDayTime self _postdawnoffset _preduskoffset))
        (if (and _isday _bcontaineractivated)
          (Variables|Default|SetManualActivationState 1)
          (elif (and (not _isday) (not _bcontaineractivated))
            (Variables|Default|SetManualActivationState -1)
            (else
              (Variables|Default|SetManualActivationState 0))))))
    (:then_2
      (return true))))

(fn CheckTime
  (bind _isdaytime (Variables|Default|GetIsDayTime))
  (bind _lightsettings (Variables|Default|GetLightSettings))
  (bind _bcontaineractivated (Variables|Default|GetbContainerActivated))
  (bind (_postdawnoffset _preduskoffset) (Utilities|Struct|BreakSPLightSettings _lightsettings))
  (bind _isday (CallFunction|SPIsDayTime self _postdawnoffset _preduskoffset))
  (Variables|Default|SetIsDaytime _isday)
  (Utilities|FlowControl|Sequence
    (:then_0
      (if (and (or (Math|Boolean|NotEqual(Boolean) _isday (Variables|Default|GetIsDaytime)) (Math|Boolean|Equal(Boolean) _isday (Variables|Default|GetbContainerActivated))) (== (Variables|Default|GetManualActivationState) 0))
        (if (Variables|Default|GetIsDayTime)
          (if _bcontaineractivated
            (Class|PrimalStructure|SetContainerActive false))
          (elif (not _bcontaineractivated)
            (Class|PrimalStructure|SetContainerActive true)))))
    (:then_1
      (if (!= (Variables|Default|GetManualActivationState) 0)
        (if (and (not _isdaytime) (== (Variables|Default|GetManualActivationState) 1))
          (Variables|Default|SetManualActivationState 0 :!label _label)
          (elif (and _isdaytime (== (Variables|Default|GetManualActivationState) -1))
            (goto _label)))))))

(fn HandleStartInterval
  (bind _lightsettings (Variables|Default|GetLightSettings))
  (if (and (Variables|Default|GetbContainerActivated) (.usesecondarycolor _lightsettings))
    (Variables|Default|SetLerpIncrement (/ 0.03333 (.secondaryinterval _lightsettings)))
    (Utilities|Time|SetTimerbyFunctionName 0 "HandleIntervalLightEvent" (Math|Float|SelectFloat (.secondaryinterval _lightsettings) 0.03333 (.doblink _lightsettings)) true)
    (else
      (Utilities|Time|ClearTimerbyFunctionName 0 "HandleIntervalLightEvent"))))

(fn HandlePrimaryColor
  (bind _lightsettings (Variables|Default|GetLightSettings))
  (Class|KismetSystemLibrary|CanRunCosmeticEvents
    (:Yes
      (CallFunction|SetActiveMaterialProperties (.r (.primarycolor _lightsettings)) (.g (.primarycolor _lightsettings)) (.b (.primarycolor _lightsettings)) (.a (.primarycolor _lightsettings)))
      (if (Variables|Default|GetbContainerActivated)
        (bind _aslamppostemitteromni_c (Utilities|Casting|CastToLampPostEmitterOmni (Variables|/Script/Engine.ChildActorComponent|GetChildActor (Variables|Default|GetActivatedEmitter))))
        (Rendering|Components|Light|SetLightColor (Variables|/Game/PrimalEarth/Test/LampPostEmitterOmni.LampPostEmitterOmni_C|GetPointLight1 _aslamppostemitteromni_c) (Utilities|Struct|MakeLinearColor (.r (.primarycolor _lightsettings)) (.g (.primarycolor _lightsettings)) (.b (.primarycolor _lightsettings)) 1.0))
        (Rendering|Components|Light|SetIntensity (Variables|/Game/PrimalEarth/Test/LampPostEmitterOmni.LampPostEmitterOmni_C|GetPointLight1 _aslamppostemitteromni_c) (.a (.primarycolor _lightsettings)))
        (Effects|Components|ParticleSystem|SetVectorParameter (Variables|/Script/Engine.Emitter|GetParticleSystemComponent _aslamppostemitteromni_c) "LightColor" (Math|Vector|MakeVector (.r (.primarycolor _lightsettings)) (.g (.primarycolor _lightsettings)) (.b (.primarycolor _lightsettings))))))))

(fn ReceiveBeginPlay
  (|CallParentFunction)
  (if (not (Variables|Default|GetbIsPreviewStructure))
    (CallFunction|HandlePrimaryColor)
    (Networking|SwitchHasAuthority
      (:Authority
        (CallFunction|HandleBeginPlayEvent)))))

(fn SetActiveMaterialProperties
  (params (R :type Float%20%28single-precision%29) (G :type Float%20%28single-precision%29) (B :type Float%20%28single-precision%29) (A :type Float%20%28single-precision%29))
  (bind _returnvalue (Math|Float|MakeLiteralFloat 5.0))
  (Rendering|Material|SetVectorParameterValue (CallFunction|GetActiveMaterial) "Emissive - Color and Intensity" (Utilities|Struct|MakeLinearColor (+ (* R A) (* R _returnvalue)) (+ (* G A) (* G _returnvalue)) (+ (* B A) (* B _returnvalue)) (Math|Float|SelectFloat 1.0 0.0 (Variables|Default|GetbContainerActivated))) :!class /Script/Engine.MaterialInstanceDynamic))

(fn GetActiveMaterial
  (bind _mystaticmesh (Variables|Default|GetMyStaticMesh))
  (Utilities|FlowControl|Sequence
    (:then_0
      (Utilities|IsValid (Variables|Default|GetActiveMaterial)
        (:Is%20Not%20Valid
          (bind _asmaterialinstancedynamic (Utilities|Casting|CastToMaterialInstanceDynamic (Rendering|Material|GetMaterial _mystaticmesh 1))
            (:then
              (Variables|Default|SetActiveMaterial _asmaterialinstancedynamic))
            (:CastFailed
              (bind _returnvalue (Rendering|Material|CreateDynamicMaterialInstance _mystaticmesh 1 0 :!class /Script/Engine.PrimitiveComponent))
              (Variables|Default|SetActiveMaterial _returnvalue))))))
    (:then_1
      (return (Variables|Default|GetActiveMaterial)))))