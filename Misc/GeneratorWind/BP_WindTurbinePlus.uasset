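; Wind turbine structure that switches itself on and off with local wind, requires open sky to place, and cannot be toggled by players.
; A randomized looping timer and unstasis trigger a sky trace and wind sample, with the server setting activation against a minimum threshold.
; Game-mode config supplies that threshold, the power range used in the water-pipe source check, and a replicated flag that mutes the active emitter's sound.
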(event Custom|ForceUpdateWind
  (CallFunction|UpdateWind))

(fn ConstructionScript
  (|CallParentFunction))

(fn BPContainerDeactivated)

(fn BPContainerActivated)

(fn BPCanbeActivated
  (return true))

(fn BPCanbeActivatedbyPlayer
  (params (PC :type Shooter%20Player%20Controller%20Object%20Reference))
  (return false))

(fn BPIsValidWaterSourceforPipe
  (params (ForWaterPipe :type Primal%20Structure%20Water%20Pipe%20Object%20Reference))
  (return (< (Math|Vector|VectorLength (- (Transformation|GetActorLocation ForWaterPipe) (Transformation|GetActorLocation))) (Variables|Default|GetMaxPowerDistance))))

(fn UpdateWind
  (bind _returnvalue (Transformation|GetActorLocation))
  (bind _returnvalue_2 (Class|Actor|GetWorld))
  (bind _returnvalue_3 (+ _returnvalue "0, 0,80.000000"))
  (if (not (Variables|Default|GetbIsPreviewStructure))
    (Utilities|FlowControl|Sequence
      (:then_0
        (bind _returnvalue_4 (Class|VictoryCore|BPFastTrace _returnvalue_2 (+ _returnvalue "0, 0,5000.000000") _returnvalue_3 self))
        (if _returnvalue_4
          (bind _returnvalue_5 (Class|PrimalGlobals|GetDayCycleManager _returnvalue_2))
          (Utilities|IsValid _returnvalue_5
            (:Is%20Valid
              (bind _returnvalue_6 (Class|DayCycleManager|GetWindatLocation _returnvalue_5 _returnvalue_3))
              (Variables|Default|SetCurrentWind _returnvalue_6)))
          (else
            (Variables|Default|SetCurrentWind 0.0))))
      (:then_1
        (if (Networking|IsServer)
          (bind _returnvalue_7 (Class|PrimalStructureItemContainer|CanbeActivated))
          (if (Math|Boolean|NotEqual(Boolean) (Variables|Default|GetbContainerActivated) (and _returnvalue_7 (>= (Variables|Default|GetCurrentWind) (Variables|Default|GetTurnOffForWindLessThan))))
            (Class|PrimalStructure|SetContainerActive (and _returnvalue_7 (>= (Variables|Default|GetCurrentWind) (Variables|Default|GetTurnOffForWindLessThan))))))))))

(fn BPUnstasis
  (CallFunction|UpdateWind))

(fn BPIsAllowedtoBuild
  (params (OutPlacementData :type Placement%20Data%20Structure%20%28by%20ref%29) (CurrentAllowedReason :type Integer))
  (bind _returnvalue (== CurrentAllowedReason -9))
  (bind _returnvalue_2 (Transformation|GetActorLocation))
  (bind _returnvalue_3 (Math|Integer|SelectInt 1 CurrentAllowedReason _returnvalue))
  (LocalVariables|SetretVal _returnvalue_3)
  (if (>= _returnvalue_3 1)
    (bind _returnvalue_4 (Class|VictoryCore|BPFastTrace (Class|Actor|GetWorld) (+ _returnvalue_2 "0, 0,4000.000000") (+ _returnvalue_2 "0, 0,50.000000") self))
    (if _returnvalue_4
      _
      (else
        (LocalVariables|SetretVal -100))))
  (return (LocalVariables|GetretVal)))

(fn BPOverrideCantBuildReasonString
  (params (CantBuildReason :type Integer))
  (if (== CantBuildReason -100)
    (LocalVariables|SetretVal "Needs open access to the sky!"))
  (return (LocalVariables|GetretVal)))

(fn BPGetMultiUseEntries
  (params (ForPC :type Player%20Controller%20Object%20Reference) (MultiUseEntries :type Array%20of%20Multi%20Use%20Entry%20Structures))
  (bind _entriesout (CallFunction|SPUpdateMultiUseMenu ForPC MultiUseEntries self false false false false))
  (return _entriesout))

(fn SetTurbineSettings
  (bind _returnvalue (Game|GetGameMode))
  (Utilities|FlowControl|Sequence
    (:then_0
      (bind _value (CallFunction|SPGetConfig-Float _returnvalue "MinWindForTurbine" 2e+01 -1.0 1e+02))
      (Variables|Default|SetTurnOffForWindLessThan (Math|Float|SelectFloat 0.0 _value (< _value 0.0)) true))
    (:then_1
      (bind _value_2 (CallFunction|SPGetConfig-Int _returnvalue "TurbineMaxPowerDistanceInFoundations" 30 1 1000))
      (Variables|Default|SetMaxPowerDistance (* _value_2 3e+02) true))))

(fn ReceiveBeginPlay
  (|CallParentFunction)
  (if (not (Variables|Default|GetbIsPreviewStructure))
    (Utilities|Time|SetTimerbyFunctionName 0 "ForceUpdateWind" (Math|Random|RandomFloatinRange 16.0 34.0) true)
    (Networking|SwitchHasAuthority
      (:Authority
        (CallFunction|SetTurbineSettings)
        (CallFunction|UpdateWind)
        (bind _disablesound (CallFunction|SPGetConfigSetting-Noise (Game|GetGameMode)))
        (Variables|Default|SetDisableSound _disablesound true)))))

(fn OnRepDisableSound
  (if (not (Networking|IsDedicatedServer))
    (if (Variables|Default|GetDisableSound)
      (bind _asprimalemitterspawnable (Utilities|Casting|CastToPrimalEmitterSpawnable (Variables|/Script/Engine.ChildActorComponent|GetChildActor (Variables|Default|GetActivatedEmitter))))
      (Audio|Components|Audio|SetVolumeMultiplier (Variables|/Script/ShooterGame.PrimalEmitterSpawnable|GetSoundToPlay _asprimalemitterspawnable) 0.0 :!class /Script/Engine.AudioComponent))))