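; BP_Incinerator is a placeable structure that destroys items put into its inventory.
; An inventory change starts a one-second looping DeleteItems timer, which force-removes items in a capped loop and clears itself on completion.
; Outside dedicated servers, it activates a particle and uses a dynamic display material whose emissive follows structure color or defaults to blue.
; Placement overrides one specific disallow reason; multi-use entries come from a shared menu helper.
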(fn `BPGetMultiUseEntries`
  (params (ForPC :type "PlayerController Object Reference") (MultiUseEntries :type "Array of Actor.MultiUseEntry Structure (by ref)"))
  (returns (ReturnValue :type "Array of Actor.MultiUseEntry Structure"))
  (bind _entriesout (`/Game/Mods/StructuresPlusMod/_Scripts/MultiUseMenuFunctions.SP_UpdateMultiUseMenu` ForPC MultiUseEntries self))
  (return _entriesout))

(fn `BPIsAllowedToBuild`
  (params (OutPlacementData :type "PrimalStructure.PlacementData Structure (by ref)") (CurrentAllowedReason :type Integer))
  (returns (ReturnValue :type Integer))
  (return (`KismetMathLibrary.SelectInt` 1 CurrentAllowedReason (== CurrentAllowedReason -9))))

(fn `BPNotifyInventoryItemChange`
  (params (bIsItemAdd :type Boolean) (theItem :type "PrimalItem Object Reference") (bEquipItem :type Boolean))
  (if (not (`KismetSystemLibrary.K2_IsTimerActive` null "DeleteItems"))
    (`KismetSystemLibrary.K2_SetTimer` null "DeleteItems" 1.0 true)))

(fn `BPRefreshedStructureColors`
  (bind _displaymat (`self.DisplayMat`))
  (if (not (`KismetSystemLibrary.IsDedicatedServer`))
    (`/Engine/EditorBlueprintResources/StandardMacros.IsValid` _displaymat
      (:`Is Valid`
        (if (`self.bUsingStructureColors`)
          (bind _returnvalue (`self.GetStructureColor` 0))
          (bind (_r _g _b) (break `Object.LinearColor` _returnvalue))
          (`MaterialInstanceDynamic.SetVectorParameterValue` _displaymat "Emissive - Color and Intensity" (make `Object.LinearColor` _r _g _b 15.0))
          (else
            (`MaterialInstanceDynamic.SetVectorParameterValue` _displaymat "Emissive - Color and Intensity" (struct :`G` 0.4 :`B` 1.0 :`A` 15.0))))))))

(fn `BPTryMultiUse`
  (params (ForPC :type "PlayerController Object Reference") (UseIndex :type Integer))
  (returns (ReturnValue :type Boolean))
  (return true))

(fn `DeleteItems`
  (bind _myinventorycomponent (`self.MyInventoryComponent`))
  (bind _inventoryitems (`PrimalInventoryComponent.InventoryItems` _myinventorycomponent))
  (`/Game/Mods/StructuresPlusMod/_Macros/UtilityMacros.SP_While` (> (`KismetArrayLibrary.Array_Length` _inventoryitems) 0) 1500
    (:`Loop Body`
      (`PrimalInventoryComponent.RemoveItem` _myinventorycomponent (`PrimalItem.ItemID` (`KismetArrayLibrary.Array_Get` _inventoryitems)) false false true false))
    (:`Completed`
      (`KismetSystemLibrary.K2_ClearTimer` null "DeleteItems"))))

(fn `ReceiveBeginPlay`
  (`parent.ReceiveBeginPlay`)
  (if (not (`self.bIsPreviewStructure`))
    (`/Engine/EditorBlueprintResources/ActorMacros.Switch Has Authority`)))

(fn `UserConstructionScript`
  (`parent.UserConstructionScript`)
  (if (not (or (`KismetSystemLibrary.IsDedicatedServer`) (`self.bIsPreviewStructure`)))
    (`ActorComponent.Activate` (`self.IncineratorParticle`) false)
    (bind _returnvalue (`KismetMaterialLibrary.CreateDynamicMaterialInstance` "/Game/Extinction/WeaponGravityGrenade/MIC_GravityGrenade.MIC_GravityGrenade"))
    (set `self.DisplayMat` _returnvalue)
    (`PrimitiveComponent.SetMaterial` (`self.DisplayMesh`) 0 _returnvalue)))