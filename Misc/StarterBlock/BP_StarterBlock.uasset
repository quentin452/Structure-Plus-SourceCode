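; BP_StarterBlock is an S+ placeable structure that players can nudge and rotate after placement, with snapped children taking its exact transform.
; Multi-use entries open triple-slider widgets whose client and server exec commands apply offsets relative to the saved placed transform, with the server storing the values.
; Position offsets follow the adjusted rotation.
; BeginPlay applies global foundation settings, dropping forced ground placement when foundations are not required.
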(fn `BPClientDoMultiUse`
  (params (ForPC :type "PlayerController Object Reference") (ClientUseIndex :type Integer))
  (`/Engine/EditorBlueprintResources/StandardMacros.IsValid` ForPC
    (:`Is Valid`
      (switch `int` ClientUseIndex
        (:`9400`
          (bind _returnvalue (`|CreateWidget` "/Game/Mods/StructuresPlusMod/_Widgets/Widget_TripleSlider.Widget_TripleSlider_C" ForPC self "Adjust Position" "" "" "" "UpdatePos_Client" "UpdatePos_Server"))
          (`/Game/Mods/StructuresPlusMod/_Widgets/Widget_TripleSlider.InitializeWidget` _returnvalue (`self.CurPosOffset`) (`self.MinPosOffset`) (`self.MaxPosOffset`))
          (`UserWidget.AddToViewport` _returnvalue))
        (:`9401`
          (bind _returnvalue_2 (`|CreateWidget` "/Game/Mods/StructuresPlusMod/_Widgets/Widget_TripleSlider.Widget_TripleSlider_C" ForPC self "Adjust Rotation" "" "" "" "UpdateRot_Client" "UpdateRot_Server"))
          (`/Game/Mods/StructuresPlusMod/_Widgets/Widget_TripleSlider.InitializeWidget` _returnvalue_2 (`self.CurRotOffset`) (`self.MinRotOffset`) (`self.MaxRotOffset`))
          (`UserWidget.AddToViewport` _returnvalue_2))))))

(fn `BPClientHandleNetExecCommand`
  (params (CommandName :type Name) (ExecParams :type "Actor.BPNetExecParams Structure (by ref)") (ForPC :type "PlayerController Object Reference"))
  (returns (ReturnValue :type Boolean))
  (bind ((`FloatParam1` _floatparam1) (`FloatParam2` _floatparam2) (`FloatParam3` _floatparam3)) (break `Actor.BPNetExecParams` ExecParams))
  (`|ExecutionSequence`
    (:`then_0`
      (`/Engine/EditorBlueprintResources/StandardMacros.IsValid` ForPC
        (:`Is Valid`
          (switch `name` CommandName
            (:`UpdatePos_Client`
              (`self.UpdatePosition` (`KismetMathLibrary.MakeVector` _floatparam1 _floatparam2 _floatparam3)))
            (:`UpdateRot_Client`
              (`self.UpdateRotation` (`KismetMathLibrary.MakeVector` _floatparam1 _floatparam2 _floatparam3)))))))
    (:`then_1`
      (return false))))

(fn `BPGetMultiUseEntries`
  (params (ForPC :type "PlayerController Object Reference") (MultiUseEntries :type "Array of Actor.MultiUseEntry Structure (by ref)"))
  (returns (ReturnValue :type "Array of Actor.MultiUseEntry Structure"))
  (bind _returnvalue (`KismetMathLibrary.Conv_LinearColorToColor` (`/Game/Mods/StructuresPlusMod/_Scripts/MultiUseMenuFunctions.SP_GetMultiUseSpecialColor`)))
  (bind _entriesout (`/Game/Mods/StructuresPlusMod/_Scripts/MultiUseMenuFunctions.SP_Update_Multi_Use_Menu` ForPC MultiUseEntries self))
  (`|ExecutionSequence`
    (:`then_0`
      (`KismetArrayLibrary.Array_Add` _entriesout (make `Actor.MultiUseEntry` :`UseString` "[Adjust Position]" :`UseIndex` 9400 :`Priority` -1006 :`bOverrideUseTextColor` true :`UseTextColor` _returnvalue))
      (`KismetArrayLibrary.Array_Add` _entriesout (make `Actor.MultiUseEntry` :`UseString` "[Adjust Rotation]" :`UseIndex` 9401 :`Priority` -1010 :`bOverrideUseTextColor` true :`UseTextColor` _returnvalue)))
    (:`then_1`
      (return _entriesout))))

(fn `BPOverrideSnappedToTransform`
  (params (childStructure :type "PrimalStructure Object Reference") (ChildSnapFromIndex :type Integer) (ChildSnapFromName :type Name) (UnsnappedPlacementPos :type "Object.Vector Structure") (UnsnappedPlacementRot :type "Object.Rotator Structure") (SnappedPlacementPos :type "Object.Vector Structure") (SnappedPlacementRot :type "Object.Rotator Structure") (SnapToIndex :type Integer) (SnapToName :type Name))
  (returns (OutLocation :type "Object.Vector Structure") (OutRotation :type "Object.Rotator Structure") (bForceInvalidateSnap :type Integer) (ReturnValue :type Boolean))
  (return (`self.K2_GetActorLocation`) (`self.K2_GetActorRotation`) 0 true))

(fn `BPPlacedStructure`
  (params (ForPC :type "PlayerController Object Reference"))
  (set `self.PlacedPos` (.location (`self.GetTransform`)) true)
  (set `self.PlacedRot` (.rotation (`self.GetTransform`)) true))

(fn `BPServerHandleNetExecCommand`
  (params (FromPC :type "PlayerController Object Reference") (CommandName :type Name) (ExecParams :type "Actor.BPNetExecParams Structure (by ref)"))
  (returns (ReturnValue :type Boolean))
  (bind ((`FloatParam1` _floatparam1) (`FloatParam2` _floatparam2) (`FloatParam3` _floatparam3)) (break `Actor.BPNetExecParams` ExecParams))
  (`|ExecutionSequence`
    (:`then_0`
      (`/Engine/EditorBlueprintResources/StandardMacros.IsValid` FromPC
        (:`Is Valid`
          (switch `name` CommandName
            (:`UpdatePos_Server`
              (`self.UpdatePosition` (`KismetMathLibrary.MakeVector` _floatparam1 _floatparam2 _floatparam3))
              (set `self.CurPosOffset` (`KismetMathLibrary.MakeVector` _floatparam1 _floatparam2 _floatparam3) true))
            (:`UpdateRot_Server`
              (`self.UpdateRotation` (`KismetMathLibrary.MakeVector` _floatparam1 _floatparam2 _floatparam3))
              (set `self.CurRotOffset` (`KismetMathLibrary.MakeVector` _floatparam1 _floatparam2 _floatparam3) true))))))
    (:`then_1`
      (return false))))

(fn `BPTryMultiUse`
  (params (ForPC :type "PlayerController Object Reference") (UseIndex :type Integer))
  (returns (ReturnValue :type Boolean))
  (return (or (== UseIndex 9400) (== UseIndex 9401))))

(fn `ReceiveBeginPlay`
  (`parent.ReceiveBeginPlay`)
  (bind _assplusglobalactor_c (cast `/Game/Mods/StructuresPlusMod/SPlusGlobalActor` (`/Game/Mods/StructuresPlusMod/_Scripts/GlobalActorFunctions.SP_GetGlobalActor` self)))
  (`/Game/Mods/StructuresPlusMod/SPlusGlobalActor.SetFoundationSettings` _assplusglobalactor_c self)
  (if (`/Game/Mods/StructuresPlusMod/SPlusGlobalActor.NoFoundationsRequired` _assplusglobalactor_c)
    (set `self.bForcePlacingOnGround` false)))

(fn `UpdatePosition`
  (params (NewOffset :type "Object.Vector Structure"))
  (bind (_currotoffset_x _currotoffset_y _currotoffset_z) (`KismetMathLibrary.BreakVector` (`self.CurRotOffset`)))
  (`self.K2_SetActorLocation` (+ (`self.PlacedPos`) (`KismetMathLibrary.GreaterGreater_VectorRotator` NewOffset (`KismetMathLibrary.ComposeRotators` (`KismetMathLibrary.MakeRot` _currotoffset_y _currotoffset_z _currotoffset_x) (`self.PlacedRot`))))))

(fn `UpdateRotation`
  (params (NewOffset :type "Object.Vector Structure"))
  (`self.SetActorRotation` (`KismetMathLibrary.ComposeRotators` (`KismetMathLibrary.MakeRot` NewOffset_Y NewOffset_Z NewOffset_X) (`self.PlacedRot`))))

(fn `UserConstructionScript`
  (`parent.UserConstructionScript`))