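; Flexible electrical wire structure that auto-connects to nearby wires within range and draws straight cable spline meshes from its center to each connection point.
; Placement preview shows the cables and blocks building without a connection point.
; On placement or a cooldown-limited "Refresh Connections" use, the server relinks neighbors and recomputes points, demolishing the wire if none remain.
; Cosmetic code rebuilds meshes, choosing material by power-source link, and hides them with the structure.
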(event Custom|RefreshConnections
  (params (PC :type Player%20Controller%20Object%20Reference))
  (Class|KismetSystemLibrary|IsRunningonServer
    (:Yes
      (bind _returnvalue (Class|StructuresPlus|SPGetNearbyStructuresforFlexibleConnection self (Variables|Default|GetSearchNearbyWireType) (Variables|Default|GetConnectionRange)))
      (if (> (Utilities|Array|Length _returnvalue) 0)
        (CallFunction|LinkWires _returnvalue)
        (bind _connectionpoints (Class|StructuresPlus|SPGetCentralPointforFlexibleConnection _returnvalue self (Variables|Default|GetDebugMode)))
        (Variables|Default|SetConnectionPoints _connectionpoints true)
        (if (> (Utilities|Array|Length _connectionpoints) 0)
          (Variables|Default|SetConnectionCenterPoint (Transformation|GetActorLocation) true)
          (CallFunction|UpdateSplineMeshesEvent)
          (else
            (CallFunction|DestroyPipe PC :!label _label)))
        (else
          (goto _label))))))

(event Custom|HideSplineMeshesEvent
  (bind _splinemeshes (Variables|Default|GetSplineMeshes))
  (if (> (Utilities|Array|Length _splinemeshes) 0)
    (for _array_element _splinemeshes
      (Rendering|SetVisibility _array_element false false))
    (else
      (Class|KismetSystemLibrary|SetTimerforNextTick 0 "HideSplineMeshesEvent" false))))

(event Custom|UpdateSplineMeshesEvent
  (Class|KismetSystemLibrary|CanRunCosmeticEvents
    (:Yes
      (CallFunction|AddSplineMeshComponents false))))

(fn ConstructionScript
  (|CallParentFunction))

(fn BPIsAllowedtoBuild
  (params (OutPlacementData :type Placement%20Data%20Structure%20%28by%20ref%29) (CurrentAllowedReason :type Integer))
  (bind _self self)
  (LocalVariables|SetBuildReason (Math|Integer|SelectInt 1 CurrentAllowedReason (== CurrentAllowedReason -9)))
  (Utilities|FlowControl|Sequence
    (:then_0
      (if (Variables|Default|GetbIsPreviewStructure)
        (bind _returnvalue (Class|StructuresPlus|SPGetNearbyStructuresforFlexibleConnection _self (Variables|Default|GetSearchNearbyWireType) (Variables|Default|GetConnectionRange)))
        (bind _connectionpoints (Class|StructuresPlus|SPGetCentralPointforFlexibleConnection _returnvalue _self (Variables|Default|GetDebugMode)))
        (Variables|Default|SetConnectionPoints _connectionpoints false)
        (Variables|Default|SetConnectionCenterPoint (.AdjustedLocation (Utilities|Struct|BreakPlacementData OutPlacementData)) false)
        (CallFunction|AddSplineMeshComponents true)
        (if (< (Utilities|Array|Length _connectionpoints) 1)
          (LocalVariables|SetBuildReason -100))))
    (:then_1
      (return (LocalVariables|GetBuildReason)))))

(fn BPOverrideCantBuildReasonString
  (params (CantBuildReason :type Integer))
  (return (Utilities|String|SelectString "Requires at least one nearby wire to connect to." "" (== CantBuildReason -100))))

(fn AddSplineMeshComponents
  (params (UsePreviewMaterial :type Boolean))
  (bind _splinemeshes (Variables|Default|GetSplineMeshes))
  (Utilities|FlowControl|Sequence
    (:then_0
      (if (> (Utilities|Array|Length _splinemeshes) 0)
        (for _array_element _splinemeshes
          (Components|DestroyComponent _array_element))
        (Utilities|Array|Clear _splinemeshes)))
    (:then_1
      (if UsePreviewMaterial
        (LocalVariables|SetMaterial_ASM "/Game/PrimalEarth/StructuresPlus/_Materials/PreviewMaterial.PreviewMaterial")
        (else
          (LocalVariables|SetMaterial_ASM (select (Class|PrimalStructure|IsLinkedtoWaterorPowerSource) (Variables|Default|GetHasWaterMaterial) (Variables|Default|GetNoWaterMaterial))))))
    (:then_2
      (for _array_element_2 (Variables|Default|GetConnectionPoints)
        (bind _returnvalue (AddComponent|AddSplineMeshComponent true))
        (Class|SceneComponent|Attachto _returnvalue (Variables|Default|GetMyRootTransform) "None" "KeepWorldPosition" true)
        (Components|StaticMesh|SetStaticMesh _returnvalue "/Game/PrimalEarth/Test_Efecto/PowerCablesStructures/SM_CablesStraight.SM_CablesStraight")
        (Transformation|SetAbsolute _returnvalue false false false)
        (SplineMesh|SetStartandEnd _returnvalue (Variables|Default|GetConnectionCenterPoint) "0, 0, 0" _array_element_2 "0, 0, 0" :!class /Script/Engine.SplineMeshComponent)
        (Rendering|Material|SetMaterial _returnvalue 0 (LocalVariables|GetMaterial_ASM))
        (Utilities|Array|Add (Variables|Default|GetSplineMeshes) _returnvalue)))))

(fn LinkWires
  (params (Connections :type Array%20of%20Primal%20Structure%20Object%20References))
  (bind _linkedstructures (Variables|Default|GetLinkedStructures))
  (Class|KismetSystemLibrary|IsRunningonServer
    (:Yes
      (for _array_element _linkedstructures
        (Utilities|Array|RemoveItem (Variables|/Script/ShooterGame.PrimalStructure|GetLinkedStructures _array_element) self))
      (Utilities|Array|Clear _linkedstructures)
      (for _array_element_2 Connections
        (Class|PrimalStructure|LinkStructure _array_element_2)))))

(fn BPGetMultiUseEntries
  (params (ForPC :type Player%20Controller%20Object%20Reference) (MultiUseEntries :type Array%20of%20Multi%20Use%20Entry%20Structures))
  (bind _canrefresh (CallFunction|IsAllowedtoRefreshConnections ForPC))
  (bind _returnvalue (|CallParentFunction ForPC MultiUseEntries))
  (Utilities|FlowControl|Sequence
    (:then_0
      (bind _returnvalue_2 (Class|PrimalStructure|AllowStructureAccess ForPC))
      (if _returnvalue_2
        (Utilities|Array|Add _returnvalue (Utilities|Struct|MakeMultiUseEntry "Refresh Connections" 771024 (Math|Integer|SelectInt 0 -5000 _canrefresh) (not _canrefresh)))))
    (:then_1
      (return _returnvalue))))

(fn IsAllowedtoRefreshConnections
  (params (PC :type Player%20Controller%20Object%20Reference))
  (Utilities|FlowControl|Sequence
    (:then_0
      (bind _asshooterplayerstate (Utilities|Casting|CastToShooterPlayerState (Variables|/Script/Engine.Controller|GetPlayerState PC)))
      (LocalVariables|SetCanRefresh_IAT (Class|ShooterPlayerState|IsAllowedtoRefreshFlexPipeConnections _asshooterplayerstate (Variables|Default|GetRefreshCooldown))))
    (:then_1
      (return (LocalVariables|GetCanRefresh_IAT)))))

(fn BPTryMultiUse
  (params (ForPC :type Player%20Controller%20Object%20Reference) (UseIndex :type Integer))
  (Utilities|FlowControl|Sequence
    (:then_0
      (Class|KismetSystemLibrary|IsRunningonServer
        (:Yes
          (switch int UseIndex
            (:771024
              (bind _returnvalue (Class|PrimalStructure|AllowStructureAccess ForPC))
              (if (and _returnvalue (CallFunction|IsAllowedtoRefreshConnections ForPC))
                (CallFunction|RefreshConnections ForPC)
                (bind _asshooterplayerstate (Utilities|Casting|CastToShooterPlayerState (Variables|/Script/Engine.Controller|GetPlayerState ForPC)))
                (Class|ShooterPlayerState|ResetFlexPipeGlobalCooldown _asshooterplayerstate)))))))
    (:then_1
      (bind _returnvalue_2 (|CallParentFunction ForPC UseIndex))
      (return _returnvalue_2))))

(fn OnRepIsHidden
  (|CallParentFunction)
  (Class|KismetSystemLibrary|CanRunCosmeticEvents
    (:Yes
      (if (and (not (Variables|Default|GetDisableHide)) (Variables|Default|GetIsHidden))
        (CallFunction|HideSplineMeshesEvent)))))

(fn BPPlacedStructure
  (params (ForPC :type Player%20Controller%20Object%20Reference))
  (CallFunction|RefreshConnections ForPC)
  (CallFunction|UpdateSplineMeshesEvent))

(fn ReceiveBeginPlay
  (|CallParentFunction)
  (if (not (Variables|Default|GetbIsPreviewStructure))
    (Class|KismetSystemLibrary|CanRunCosmeticEvents
      (:Yes
        (CallFunction|AddSplineMeshComponents false)))))

(fn DestroyPipe
  (params (PC :type Player%20Controller%20Object%20Reference))
  (Utilities|IsValid PC
    (:Is%20Valid
      (Class|PrimalStructure|Demolish PC PC))
    (:Is%20Not%20Valid
      (Actor|DestroyActor))))