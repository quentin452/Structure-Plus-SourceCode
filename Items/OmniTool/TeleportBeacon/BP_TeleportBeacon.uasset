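; Teleport beacon for the OmniTool, a temporary actor that carries an owning player, team and display name.
; InitializeBeacon stores that identity, registers the beacon in the SplusTeleporterBeacon custom actor list, starts a lifespan timer and forces a net update.
; When the timer expires, SelfDestruct removes it from the list and destroys the actor.
; Shortly after BeginPlay, the authority destroys the beacon's inventory component.
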(event `self.ReceiveBeginPlay`
  (`KismetSystemLibrary.Delay` 0.2)
  (`/Engine/EditorBlueprintResources/ActorMacros.Switch Has Authority`
    (:`Authority`
      (`ActorComponent.K2_DestroyComponent` (`self.MyInventoryComponent`)))))

(event `InitializeBeacon`
  (params (Owner :type "PlayerController Object Reference") (OwnerTeam :type Integer) (BeaconName :type String) (Lifespan :type "Float (double-precision)"))
  (set `self.OwningPC` Owner)
  (set `self.TargetingTeam` OwnerTeam false)
  (set `self.DescriptiveName` BeaconName)
  (`/Game/Mods/StructuresPlusMod/_Scripts/ActorFunctions.SP_AddToCustomActorList` self "SplusTeleporterBeacon")
  (`KismetSystemLibrary.K2_SetTimerDelegate` (delegate `SelfDestruct`) Lifespan)
  (`self.ForceNetUpdate` false))

(event `SelfDestruct`
  (`|ExecutionSequence`
    (:`then_0`
      (bind _returnvalue (`VictoryCore.GetCustomActorList` (`self.K2_GetWorld`) "SplusTeleporterBeacon"))
      (`/Engine/EditorBlueprintResources/StandardMacros.IsValid` _returnvalue
        (:`Is Valid`
          (`KismetArrayLibrary.Array_RemoveItem` (`CustomActorList.ActorList` _returnvalue) self))))
    (:`then_1`
      (`self.K2_DestroyActor`))))

(fn `UserConstructionScript`
  (`parent.UserConstructionScript`))