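; Shared function library that lets players install quality blueprints into a structure's inventory as always-learned engrams, or reclaim them.
; A context-sensitive inventory button sends net exec commands from the client to toggle the selected blueprint or the display of vanilla engrams.
; Installing flips item flags, overrides the engram requirement and records it in SavedBPs.
; Helpers hide matching base-quality engrams, re-add saved blueprints on load and release them.
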(fn SPBPIntegration-AddMultiUseEntries
  (params (PC :type Player%20Controller%20Object%20Reference) (Entries :type Array%20of%20Multi%20Use%20Entry%20Structures) (UseIndex :type Integer) (ShowVanillaEngrams :type Boolean) (SavedBPs :type Array%20of%20Primal%20Item%20Object%20References))
  (Utilities|FlowControl|Sequence
    (:then_0
      (bind _asshooterplayercontroller (Utilities|Casting|CastToShooterPlayerController PC))
      (if (Pawn|IsLocalPlayerController _asshooterplayercontroller)
        (Utilities|FlowControl|Sequence
          (:then_0
            (bind _returnvalue (Class|ShooterPlayerController|GetInventoryUISelectedItemRemote _asshooterplayercontroller))
            (Utilities|IsValid _returnvalue
              (:Is%20Valid
                (if (SPFunctions_-_BP_Integration|SPBPIntegration-IsItemValid _returnvalue false)
                  (if (Variables|/Script/ShooterGame.PrimalItem|GetbIsEngram _returnvalue)
                    (LocalVariables|SetButtonString_AMU "Reclaim Blueprint")
                    (LocalVariables|SetHasItemSelected_AMU true)
                    (elif (SPFunctions_-_BP_Integration|SPBPIntegration-IsItemValid _returnvalue true)
                      (LocalVariables|SetButtonString_AMU "Install Blueprint")
                      (LocalVariables|SetHasItemSelected_AMU true)))))))
          (:then_1
            (if (and (not (LocalVariables|GetHasItemSelected_AMU)) (> (Utilities|Array|Length SavedBPs) 0))
              (LocalVariables|SetAddButton_AMU true)
              (LocalVariables|SetButtonString_AMU (Utilities|String|SelectString "Show Only Quality Engrams" "Show All Engrams" ShowVanillaEngrams)))))
        (else
          (LocalVariables|SetAddButton_AMU true))))
    (:then_1
      (if (or (LocalVariables|GetHasItemSelected_AMU) (LocalVariables|GetAddButton_AMU))
        (Utilities|Array|Add Entries (Utilities|Struct|MakeMultiUseEntry (LocalVariables|GetButtonString_AMU) UseIndex -9900 true true))))))

(fn SPBPIntegration-ClientDoMultiUse
  (params (PC :type Player%20Controller%20Object%20Reference) (Structure :type Primal%20Structure%20Item%20Container%20Object%20Reference))
  (Utilities|FlowControl|Sequence
    (:then_0
      (bind _asshooterplayercontroller (Utilities|Casting|CastToShooterPlayerController PC))
      (bind _returnvalue (Class|ShooterPlayerController|GetInventoryUISelectedItemRemote _asshooterplayercontroller))
      (Utilities|IsValid _returnvalue
        (:Is%20Valid
          (if (SPFunctions_-_BP_Integration|SPBPIntegration-IsItemValid _returnvalue false)
            (LocalVariables|SetFoundValidItem_DMU true)
            (bind (_itemid1 _itemid2) (Class|PrimalItem|BPGetItemID _returnvalue))
            (Class|PlayerController|ClientSendNetExecCommandtoServer _asshooterplayercontroller Structure "ToggleEngramStatus" (Utilities|Struct|MakeBPNetExecParams _itemid1 _itemid2) true)))))
    (:then_1
      (if (not (LocalVariables|GetFoundValidItem_DMU))
        (Class|PlayerController|ClientSendNetExecCommandtoServer PC Structure "ToggleVanillaEngrams" (Utilities|Struct|MakeBPNetExecParams) true)))))

(fn SPBPIntegration-ToggleEngramStatus
  (params (Item :type Primal%20Item%20Object%20Reference) (SavedBPs :type Array%20of%20Primal%20Item%20Object%20References) (Inventory :type Primal%20Inventory%20Component%20Object%20Reference) (ShowVanillaEngrams :type Boolean))
  (bind _returnvalue (not ShowVanillaEngrams))
  (if (SPFunctions_-_BP_Integration|SPBPIntegration-IsItemValid Item false)
    (Utilities|FlowControl|Sequence
      (:then_0
        (if (Variables|/Script/ShooterGame.PrimalItem|GetbIsEngram Item)
          (SPFunctions_-_BP_Integration|SPBPIntegration-UpdateSavedBP Item false)
          (Utilities|Array|RemoveItem SavedBPs Item)
          (LocalVariables|SetDidSomething_TES -1)
          (elif (SPFunctions_-_BP_Integration|SPBPIntegration-IsItemValid Item true)
            (SPFunctions_-_BP_Integration|SPBPIntegration-UpdateSavedBP Item true)
            (Utilities|Array|Add SavedBPs Item)
            (LocalVariables|SetDidSomething_TES 1))))
      (:then_1
        (if (!= (LocalVariables|GetDidSomething_TES) 0)
          (bind _array_element (Utilities|Array|ForEachLoopwithBreak (Variables|/Script/ShooterGame.PrimalInventoryComponent|GetInventoryItems Inventory) :!label _label)
            (:LoopBody
              (if (and (== (Utilities|GetClass _array_element) (Utilities|GetClass Item)) (== (Variables|/Script/ShooterGame.PrimalItem|GetItemQualityIndex _array_element) 0))
                (LocalVariables|SetVanillaItem_TES _array_element)
                (goto _label Break)))
            (:Completed
              (Utilities|IsValid (LocalVariables|GetVanillaItem_TES)
                (:Is%20Valid
                  (Utilities|FlowControl|Sequence
                    (:then_0
                      (if (< (LocalVariables|GetDidSomething_TES) 0)
                        (bind _array_element_2 (Utilities|Array|ForEachLoopwithBreak SavedBPs :!label _label_2)
                          (:LoopBody
                            (if (== (Utilities|GetClass _array_element_2) (Utilities|GetClass Item))
                              (LocalVariables|SetHasMoreBPs_TES true)
                              (goto _label_2 Break)))
                          (:Completed
                            (if (not (LocalVariables|GetHasMoreBPs_TES))
                              (Variables|/Script/ShooterGame.PrimalItem|SetbHideFromInventoryDisplay (LocalVariables|GetVanillaItem_TES) false)
                              (Variables|/Script/ShooterGame.PrimalItem|SetbHideFromRemoteInventoryDisplay (LocalVariables|GetVanillaItem_TES) false)
                              (Class|PrimalItem|UpdatedItem (LocalVariables|GetVanillaItem_TES) false)
                              (else
                                (Variables|/Script/ShooterGame.PrimalItem|SetbHideFromInventoryDisplay (LocalVariables|GetVanillaItem_TES) _returnvalue :!label _label_3)
                                (Variables|/Script/ShooterGame.PrimalItem|SetbHideFromRemoteInventoryDisplay (LocalVariables|GetVanillaItem_TES) _returnvalue)
                                (Class|PrimalItem|UpdatedItem (LocalVariables|GetVanillaItem_TES) false)))))))
                    (:then_1
                      (if (> (LocalVariables|GetDidSomething_TES) 0)
                        (goto _label_3)))))))))))))

(fn SPBPIntegration-ToggleVanillaEngrams
  (params (Show :type Boolean) (Structure :type Primal%20Structure%20Item%20Container%20Object%20Reference) (SavedBPs :type Array%20of%20Primal%20Item%20Object%20References))
  (bind _returnvalue (not Show))
  (for _array_element SavedBPs
    (Utilities|Array|AddUnique (LocalVariables|GetVanillaClasses_TVE) (Utilities|GetClass _array_element)))
  (for _array_element_2 (LocalVariables|GetVanillaClasses_TVE)
    (bind _array_element_3 (Utilities|Array|ForEachLoopwithBreak (Variables|/Script/ShooterGame.PrimalInventoryComponent|GetInventoryItems (Variables|/Script/ShooterGame.PrimalStructureItemContainer|GetMyInventoryComponent Structure)) :!label _label)
      (:LoopBody
        (if (and (== (Utilities|GetClass _array_element_3) _array_element_2) (== (Variables|/Script/ShooterGame.PrimalItem|GetItemQualityIndex _array_element_3) 0))
          (Variables|/Script/ShooterGame.PrimalItem|SetbHideFromInventoryDisplay _array_element_3 _returnvalue)
          (Variables|/Script/ShooterGame.PrimalItem|SetbHideFromRemoteInventoryDisplay _array_element_3 _returnvalue)
          (Class|PrimalItem|UpdatedItem _array_element_3 false)
          (goto _label Break))))))

(fn SPBPIntegration-UpdateSavedBP
  (params (SavedBP :type Primal%20Item%20Object%20Reference) (MakeEngram :type Boolean))
  (Utilities|FlowControl|Sequence
    (:then_0
      (Variables|/Script/ShooterGame.PrimalItem|SetbIsEngram SavedBP MakeEngram)
      (Variables|/Script/ShooterGame.PrimalItem|SetbAllowRemovalFromInventory SavedBP (not MakeEngram))
      (Variables|/Script/ShooterGame.PrimalItem|SetbHideFromInventoryDisplay SavedBP false)
      (Variables|/Script/ShooterGame.PrimalItem|SetbHideFromRemoteInventoryDisplay SavedBP false)
      (Variables|/Script/ShooterGame.PrimalItem|SetbAlwaysLearnedEngram SavedBP MakeEngram)
      (Variables|/Script/ShooterGame.PrimalItem|SetbForceDisplayInInventory SavedBP MakeEngram)
      (Variables|/Script/ShooterGame.PrimalItem|SetEngramRequirementItemClassOverride SavedBP (select MakeEngram "/Game/PrimalEarth/CoreBlueprints/Weapons/PrimalItem_WeaponTorch.PrimalItem_WeaponTorch_C" 0)))
    (:then_1
      (Class|PrimalItem|UpdatedItem SavedBP false))))

(fn SPBPIntegration-IsItemValid
  (params (Item :type Primal%20Item%20Object%20Reference) (ToMakeAnEngram :type Boolean))
  (Utilities|FlowControl|Sequence
    (:then_0
      (if ToMakeAnEngram
        (if (and (== (Variables|/Script/ShooterGame.PrimalItem|GetBlueprintAllowMaxCraftings Item) 0) (== (Utilities|Array|Length (Variables|/Script/ShooterGame.PrimalItem|GetCustomItemDatas Item)) 0))
          (LocalVariables|SetIsValid_IIV true :!label _label))
        (elif (and (> (Variables|/Script/ShooterGame.PrimalItem|GetItemQualityIndex Item) 0) (Variables|/Script/ShooterGame.PrimalItem|GetbIsBlueprint Item))
          (goto _label))))
    (:then_1
      (return (LocalVariables|GetIsValid_IIV)))))

(fn SPBPIntegration-LoadfromSave
  (params (Inventory :type Primal%20Inventory%20Component%20Object%20Reference) (SavedBPs :type Array%20of%20Primal%20Item%20Object%20References) (ShowVanilla :type Boolean))
  (if (> (Utilities|Array|Length SavedBPs) 0)
    (if ShowVanilla
      (SPFunctions_-_BP_Integration|SPBPIntegration-AddSavedBPs Inventory SavedBPs)
      (else
        (bind (_item _index) (Utilities|SPforEachReverse SavedBPs)
          (:Loop
            (Utilities|IsValid _item
              (:Is%20Valid
                (Utilities|Array|AddUnique (LocalVariables|GetItemClasses_LFS) (Utilities|GetClass _item)))
              (:Is%20Not%20Valid
                (Utilities|Array|RemoveIndex SavedBPs _index))))
          (:Completed
            (for _array_element (LocalVariables|GetItemClasses_LFS)
              (bind _asprimalitem (Utilities|Casting|CastToPrimalItemClass _array_element))
              (bind _returnvalue (Class|PrimalInventoryComponent|BPGetItemOfTemplate Inventory _asprimalitem false false false false true false false false true false))
              (Utilities|IsValid _returnvalue
                (:Is%20Valid
                  (if (and (Variables|/Script/ShooterGame.PrimalItem|GetbIsEngram _returnvalue) (== (Variables|/Script/ShooterGame.PrimalItem|GetItemQualityIndex _returnvalue) 0))
                    (Variables|/Script/ShooterGame.PrimalItem|SetbHideFromInventoryDisplay _returnvalue true)
                    (Variables|/Script/ShooterGame.PrimalItem|SetbHideFromRemoteInventoryDisplay _returnvalue true)
                    (Class|PrimalItem|UpdatedItem _returnvalue false)))))
            (SPFunctions_-_BP_Integration|SPBPIntegration-AddSavedBPs Inventory SavedBPs)))))))

(fn SPBPIntegration-AddSavedBPs
  (params (Inventory :type Primal%20Inventory%20Component%20Object%20Reference) (SavedBPs :type Array%20of%20Primal%20Item%20Object%20References))
  (bind (_item _index) (Utilities|SPforEachReverse SavedBPs)
    (:Loop
      (Utilities|IsValid _item
        (:Is%20Valid
          (bind _returnvalue (Class|PrimalInventoryComponent|AddItemObject Inventory _item))
          (Utilities|IsValid _returnvalue
            (:Is%20Valid
              (Variables|/Script/ShooterGame.PrimalItem|SetbAlwaysLearnedEngram _returnvalue true)
              (Variables|/Script/ShooterGame.PrimalItem|SetbForceDisplayInInventory _returnvalue true)
              (Variables|/Script/ShooterGame.PrimalItem|SetEngramRequirementItemClassOverride _returnvalue "/Game/PrimalEarth/CoreBlueprints/Weapons/PrimalItem_WeaponTorch.PrimalItem_WeaponTorch_C")
              (Class|PrimalItem|UpdatedItem _returnvalue false))))
        (:Is%20Not%20Valid
          (Utilities|Array|RemoveIndex SavedBPs _index))))))

(fn SPBPIntegration-ReleaseBPs
  (params (SavedBPs :type Array%20of%20Primal%20Item%20Object%20References))
  (for _array_element SavedBPs
    (Variables|/Script/ShooterGame.PrimalItem|SetbIsEngram _array_element false)
    (Variables|/Script/ShooterGame.PrimalItem|SetbAllowRemovalFromInventory _array_element true)))